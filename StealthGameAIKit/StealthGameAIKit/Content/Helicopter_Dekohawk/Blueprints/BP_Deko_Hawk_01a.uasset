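; Dekohawk helicopter that flies on pitch, roll and throttle values and also serves as the end-game escape trigger.
; Tick sets physics velocity, banks and yaws the body, and drives engine and door audio plus Anim Blueprint rotors and sliding doors.
; The player character overlapping EscapeBox once hides the HUD, plays the ending sequence, shows the game-clear screen and destroys the player.
; Construction assigns materials and enables in-editor animation.
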(event OnComponentBeginOverlap(EscapeBox)
  (params (OverlappedComponent :type Primitive%20Component%20Object%20Reference) (OtherActor :type Actor%20Object%20Reference) (OtherComp :type Primitive%20Component%20Object%20Reference) (OtherBodyIndex :type Integer) (bFromSweep :type Boolean) (SweepResult :type Hit%20Result%20Structure%20%28by%20ref%29))
  (if (== OtherActor (Game|GetPlayerCharacter 0))
    (Utilities|FlowControl|DoOnce false
      (:Completed
        (bind _asbp_player (Utilities|Casting|CastToBP_Player (Game|Player|GetPlayerPawn 0)))
        (bind _asbp_player_2 (Utilities|Casting|CastToBP_Player (Game|Player|GetPlayerPawn 0)))
        (Widget|SetVisibility (Variables|/Game/StealthGameAIKit/Characters/Player/BP_Player.BP_Player_C|GetMainWidget _asbp_player_2) "Hidden")
        (Pawn|Components|CharacterMovement|SetMovementMode (Variables|/Script/Engine.Character|GetCharacterMovement _asbp_player) "MOVE_None" 0)
        (bind _returnvalue (Sequencer|Player|CreateLevelSequencePlayer "/Game/Cinematics/EndGameSequence.EndGameSequence"))
        (Sequencer|Player|Play _returnvalue :!class /Script/MovieScene.MovieSceneSequencePlayer)
        (bind _returnvalue_2 (UserInterface|CreateWidget "/Game/StealthGameAIKit/UserInterface/WBP_GameOverAndClearScreen.WBP_GameOverAndClearScreen_C" (Game|GetPlayerController 0) true))
        (UserInterface|Viewport|AddtoViewport _returnvalue_2 0)
        (Actor|DestroyActor _asbp_player)))))

(event EventBeginPlay
  (bind _asabp_deko_hawk_01a (Utilities|Casting|CastToABP_Deko_Hawk_01a (Components|SkeletalMesh|GetAnimInstance (Variables|Default|GetDekogonHawk))))
  (Variables|Animation|SetABP_Deko_Hawk _asabp_deko_hawk_01a))

(event EventTick
  (params (DeltaSeconds :type Float%20%28single-precision%29))
  (bind _returnvalue (Transformation|GetActorRotation))
  (bind _returnvalue_2 (Transformation|GetVelocity))
  (bind _returnvalue_3 (Input|AxisValues|GetRoll))
  (bind _returnvalue_4 (Input|AxisValues|GetPitch))
  (bind _returnvalue_5 (Input|AxisValues|GetThrottle))
  (bind _sc_dekohawk_doors (Variables|Default|GetSC_DekoHawk_Doors))
  (bind _sc_dekohawk_engine (Variables|Default|GetSC_DekoHawk_Engine))
  (bind _abp_deko_hawk (Variables|Animation|GetABP_Deko_Hawk))
  (bind _abp_deko_hawk_2 (Variables|Animation|GetABP_Deko_Hawk))
  (bind _returnvalue_6 (Math|Vector|VectorLength _returnvalue_2))
  (bind _returnvalue_7 (* _returnvalue_5 1e+01))
  (bind _returnvalue_8 (* _returnvalue_4 -25.0))
  (bind _returnvalue_9 (* _returnvalue_3 2e+01))
  (bind _returnvalue_10 (Math|Float|Absolute(Float) _returnvalue_6))
  (bind _returnvalue_11 (+ _returnvalue_8 _returnvalue_7))
  (bind _returnvalue_12 (Math|Rotator|MakeRotator _returnvalue_9 _returnvalue_11 0.0))
  ;[1 1 1] Heli Movement
  (CallFunction|SetAnimationParameters)
  (Variables|Animation|SetDelta%20seconds DeltaSeconds)
  (Physics|SetPhysicsLinearVelocity (Variables|Default|GetPhysicsObject) (+ (Transformation|GetVelocity) (* (* (Math|Vector|RotateVector (Math|Vector|MakeVector (Input|AxisValues|GetPitch) (Input|AxisValues|GetRoll) (Input|AxisValues|GetThrottle)) (Math|Rotator|MakeRotator 0.0 0.0 (.yaw (Transformation|GetActorRotation)))) (Variables|Animation|GetMovement%20speed)) (Variables|Animation|GetDelta%20seconds))) false "None")
  (Transformation|SetActorRotation (Math|Interpolation|RInterpTo (Math|Rotator|MakeRotator (.roll _returnvalue) (.pitch _returnvalue) (.yaw _returnvalue)) (Math|Rotator|MakeRotator (.roll _returnvalue_12) (.pitch _returnvalue_12) (+ (.yaw _returnvalue) (* (Variables|Animation|GetRotation%20Speed) (Input|AxisValues|GetRoll)))) (Variables|Animation|GetDelta%20seconds) 1.0)) ; Rotate the helicopter yaw to match the camera, while pitch and roll are determined by input direction
  ;[1 1 1] Audio&Animation
  (Audio|Parameter|SetFloatParameter _sc_dekohawk_engine "Throttle" _returnvalue_10 :!class /Script/Engine.AudioComponent)
  (Audio|Components|Audio|SetPitchMultiplier _sc_dekohawk_engine (* (+ (/ _returnvalue_10 9e+03) 0.2) 3.0))
  (Variables|/Game/Helicopter_Dekohawk/Blueprints/ABP_Deko_Hawk_01a.ABP_Deko_Hawk_01a_C|SetLeftDoorLoc _abp_deko_hawk (Math|Interpolation|FInterpTo (Variables|/Game/Helicopter_Dekohawk/Blueprints/ABP_Deko_Hawk_01a.ABP_Deko_Hawk_01a_C|GetLeftDoorLoc _abp_deko_hawk) (Math|Float|SelectFloat 155.0 0.0 (Variables|Animation|GetLeftDoorOpen?)) (Utilities|Time|GetWorldDeltaSeconds) 3.7))
  (Variables|/Game/Helicopter_Dekohawk/Blueprints/ABP_Deko_Hawk_01a.ABP_Deko_Hawk_01a_C|SetRightDoorLoc _abp_deko_hawk (Math|Interpolation|FInterpTo (Variables|/Game/Helicopter_Dekohawk/Blueprints/ABP_Deko_Hawk_01a.ABP_Deko_Hawk_01a_C|GetRightDoorLoc _abp_deko_hawk) (Math|Float|SelectFloat 155.0 0.0 (Variables|Animation|GetRightDoorOpen?)) (Utilities|Time|GetWorldDeltaSeconds) 3.7))
  (Audio|Parameter|SetFloatParameter _sc_dekohawk_doors "DoorLocation0" (Variables|/Game/Helicopter_Dekohawk/Blueprints/ABP_Deko_Hawk_01a.ABP_Deko_Hawk_01a_C|GetLeftDoorLoc _abp_deko_hawk_2) :!class /Script/Engine.AudioComponent)
  (Audio|Parameter|SetFloatParameter _sc_dekohawk_doors "DoorLocation1" (Variables|/Game/Helicopter_Dekohawk/Blueprints/ABP_Deko_Hawk_01a.ABP_Deko_Hawk_01a_C|GetRightDoorLoc _abp_deko_hawk_2) :!class /Script/Engine.AudioComponent)
  (Effects|Components|ParticleSystem|SetBoolParameter _sc_dekohawk_doors "DoorSlide0" (Variables|Animation|GetLeftDoorOpen?))
  (Effects|Components|ParticleSystem|SetBoolParameter _sc_dekohawk_doors "DoorSlide1" (Variables|Animation|GetRightDoorOpen?))
  (bind _velocity (Timeline|RotationPropeller Play)
    (:Update
      (Variables|/Game/Helicopter_Dekohawk/Blueprints/ABP_Deko_Hawk_01a.ABP_Deko_Hawk_01a_C|SetLargePropellerRot _abp_deko_hawk_2 _velocity)
      (Variables|/Game/Helicopter_Dekohawk/Blueprints/ABP_Deko_Hawk_01a.ABP_Deko_Hawk_01a_C|SetSmallPropellerRot _abp_deko_hawk_2 _velocity))))

(fn ConstructionScript
  (bind _dekogonhawk (Variables|Default|GetDekogonHawk))
  (Rendering|Material|SetMaterial _dekogonhawk 2 (Variables|Material|GetHawk%20Material%20a))
  (Rendering|Material|SetMaterial _dekogonhawk 0 (Variables|Material|GetHawk%20Material%20b))
  (Rendering|Material|SetMaterial _dekogonhawk 3 (Variables|Material|GetHawk%20Material%20c))
  (Rendering|Material|SetMaterial _dekogonhawk 1 (Variables|Material|GetGlass%20Material))
  (CallFunction|InitAnimationBP)
  (if (not (Class|KismetSystemLibrary|TimerExists 0 "setAnimationParameters"))
    (Utilities|Time|SetTimerbyFunctionName self "setAnimationParameters" 0.016667 true)))

(fn SetAnimationParameters
  (Variables|/Game/Helicopter_Dekohawk/Blueprints/ABP_Deko_Hawk_01a.ABP_Deko_Hawk_01a_C|SetLpropellerSpeed (Variables|Animation|GetABP_Deko_Hawk) (Variables|Animation|customAnimation|GetLPropellerSpeed)))

(fn InitAnimationBP
  (bind _asabp_deko_hawk_01a (Utilities|Casting|CastToABP_Deko_Hawk_01a (Components|SkeletalMesh|GetAnimInstance (Variables|Default|GetDekogonHawk))))
  (Variables|Animation|SetABP_Deko_Hawk _asabp_deko_hawk_01a)
  (Components|SkeletalMesh|SetUpdateAnimationinEditor (Variables|Default|GetDekogonHawk) true))