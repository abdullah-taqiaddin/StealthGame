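; BP_briefcase is a lootable briefcase actor in the bank vault content, with an overlap box and a marker widget that starts hidden.
; Entering the box registers the briefcase on a BP_BaseCharacter, enables looting and shows a newly created loot widget.
; Leaving clears that state and removes the widget, but only for BP_Player.
; Each tick passes the marker's world location to WBP_Marker to update its text.
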(event OnComponentBeginOverlap(Box)
  (params (OverlappedComponent :type Primitive%20Component%20Object%20Reference) (OtherActor :type Actor%20Object%20Reference) (OtherComp :type Primitive%20Component%20Object%20Reference) (OtherBodyIndex :type Integer) (bFromSweep :type Boolean) (SweepResult :type Hit%20Result%20Structure%20%28by%20ref%29))
  (bind _asbp_base_character (Utilities|Casting|CastToBP_BaseCharacter OtherActor))
  (Variables|/Game/StealthGameAIKit/Characters/Base/BP_BaseCharacter.BP_BaseCharacter_C|SetBriefcase _asbp_base_character self)
  (Variables|/Game/StealthGameAIKit/Characters/Base/BP_BaseCharacter.BP_BaseCharacter_C|SetCanLoot _asbp_base_character true)
  (bind _returnvalue (UserInterface|CreateWidget "/Game/StealthGameAIKit/UserInterface/WBP_LootWidget.WBP_LootWidget_C"))
  (bind _output_get (Variables|Default|SetLootWidget _returnvalue))
  (UserInterface|Viewport|AddtoViewport _output_get 0)
  (Variables|/Game/StealthGameAIKit/Characters/Base/BP_BaseCharacter.BP_BaseCharacter_C|SetLootWidget _asbp_base_character (Variables|Default|GetLootWidget)))

(event OnComponentEndOverlap(Box)
  (params (OverlappedComponent :type Primitive%20Component%20Object%20Reference) (OtherActor :type Actor%20Object%20Reference) (OtherComp :type Primitive%20Component%20Object%20Reference) (OtherBodyIndex :type Integer))
  (bind _asbp_player (Utilities|Casting|CastToBP_Player OtherActor))
  (Variables|/Game/StealthGameAIKit/Characters/Base/BP_BaseCharacter.BP_BaseCharacter_C|SetBriefcase _asbp_player 0)
  (Variables|/Game/StealthGameAIKit/Characters/Base/BP_BaseCharacter.BP_BaseCharacter_C|SetCanLoot _asbp_player false)
  (Widget|RemovefromParent (Variables|Default|GetLootWidget)))

(event EventBeginPlay
  (Rendering|SetVisibility (Variables|Default|GetMarkerWidget) false false))

(event Collision|EventActorBeginOverlap
  (params (OtherActor :type Actor%20Object%20Reference)))

(event EventTick
  (params (DeltaSeconds :type Float%20%28single-precision%29))
  (bind _markerwidget (Variables|Default|GetMarkerWidget))
  (bind _aswbp_marker (Utilities|Casting|CastToWBP_Marker (UserInterface|GetWidget _markerwidget)))
  (Default|UpdateText _aswbp_marker (Transformation|GetWorldLocation _markerwidget)))

(fn ConstructionScript)