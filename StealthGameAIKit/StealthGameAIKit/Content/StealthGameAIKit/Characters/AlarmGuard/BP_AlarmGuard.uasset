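; Alarm guard AI character that, when its WasSeen event fires, runs to its linked Alarm actor to raise the alarm.
; It pauses its brain logic, moves to the alarm, then once plays a timed alarm sound there and restarts its logic.
; SquadAI broadcasts the player pawn as a found enemy to guards within a very large radius.
; The construction script registers this guard on the assigned Alarm.
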(event EventBeginPlay
  (|CallParentFunction) ; This node is disabled and will not be called.\nDrag off pins to build functionality.
)

(event Collision|EventActorBeginOverlap
  (params (OtherActor :type Actor%20Object%20Reference)))

(event EventWasSeen
  (params (Instigator :type BP%20Base%20Character%20Object%20Reference))
  (bind _self self)
  (bind _self_2 self)
  (bind _alarm (Variables|Default|GetAlarm))
  (bind _returnvalue (AI|GetAIController _self_2))
  (AI|Logic|StopLogic (Variables|/Script/AIModule.AIController|GetBrainComponent (AI|GetAIController _self)) "")
  (AI|AIMoveTo (AI|GetAIController _self) (Transformation|GetActorLocation _alarm) _alarm 1e+02 "Default" "Default" true true
    (:OnMoveFinished
      (Utilities|FlowControl|DoOnce false
        (:Completed
          (bind _asbp_player (Utilities|Casting|CastToBP_Player (Game|Player|GetPlayerPawn 0)))
          ;[1 1 1] Set alarm and notify guards
          (CallFunction|SetAlarmandNotifyGuards _asbp_player)
          (Utilities|Casting|CastToAIC_Guard _returnvalue)
          (Class|BrainComponent|RestartLogic (Variables|/Script/AIModule.AIController|GetBrainComponent _returnvalue)))))))

(fn ConstructionScript
  (bind _alarm (Variables|Default|GetAlarm))
  (|CallParentFunction)
  (Utilities|IsValid _alarm
    (:Is%20Valid
      (Variables|/Game/StealthGameAIKit/Interactable/BP_Alarm.BP_Alarm_C|SetGuard _alarm self))))

(fn SetAlarmandNotifyGuards
  (params (Player :type BP%20Player%20Object%20Reference))
  (bind _self self)
  (bind _returnvalue (Audio|SpawnSoundatLocation "/Game/StealthGameAIKit/Sound/Alarm.Alarm" (Transformation|GetActorLocation (Variables|Default|GetAlarm)) "0, 0, 0" 1.0 1.0 0.0 0 0))
  (Audio|Components|Audio|StopDelayed _returnvalue 18.0)
  (bind _asaic_guard (Utilities|Casting|CastToAIC_Guard (AI|GetAIController self)))
  (Default|NotifyFindEnemy (Variables|/Game/StealthGameAIKit/Characters/GuardAI/BP_Guard.BP_Guard_C|GetSquadAI _self) _self _asaic_guard 2e+05 Player))