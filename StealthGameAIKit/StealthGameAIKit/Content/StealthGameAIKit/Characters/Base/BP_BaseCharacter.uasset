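; Base character for the stealth AI kit, handling health, weapons, aiming, reloading and death.
; It spawns default weapons on BeginPlay, equips and reloads them through montages, and broadcasts state changes via dispatchers.
; Point damage reduces health, with head or neck hits calling death directly; death stops guard AI, unpossesses and ragdolls with a timer-driven capsule follow.
; V and L keys save and load health, weapons, location, guard states and collected keys.
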(event Custom|EquipWeapon
  (params (WeaponIndex :type Integer))
  ;[1 1 1] Equip Weapon
  (Variables|Weapon|SetNewWeaponIndex WeaponIndex)
  (if (<= (Variables|Weapon|GetNewWeaponIndex) (Utilities|Array|LastIndex (Variables|Weapon|GetWeaponInventory)))
    (if (and (!= (Variables|Weapon|GetNewWeaponIndex) (Variables|Weapon|GetCurrentWeaponIndex)) (not (Variables|Weapon|GetbReloading)))
      (Variables|Weapon|SetCurrentWeaponIndex (Variables|Weapon|GetNewWeaponIndex))
      (bind _currentweapon (Variables|Weapon|GetCurrentWeapon)
        (:then
          (Default|UnEquipped _currentweapon))
        (:else
          _))
      (Variables|Weapon|SetCurrentWeapon (Utilities|Array|Get(acopy) (Variables|Weapon|GetWeaponInventory) (Variables|Weapon|GetNewWeaponIndex)))
      (Default|Equipped (Variables|Weapon|GetCurrentWeapon))
      (Animation|Montage|PlayMontage (Variables|Character|GetMesh) "/Game/StealthGameAIKit/Characters/Common/Animations/AM_Equip_Pistol_Standing.AM_Equip_Pistol_Standing" 2.0
        (:OnNotifyBegin
          (Default|CallOnSwitchWeaponFinished (Variables|Weapon|GetCurrentWeapon)))))))

(event Custom|ReloadWeapon
  ;[1 1 1] Play Reload Montage
  (Variables|Weapon|SetbReloading true)
  (Utilities|IsValid (Variables|/Game/StealthGameAIKit/Weapons/Base/BP_BaseWeapon.BP_BaseWeapon_C|GetReloadMontage (Variables|Weapon|GetCurrentWeapon))
    (:Is%20Valid
      (Default|CallOnBeginReload)
      (Utilities|FlowControl|DoOnce false :!label _label
        (:Completed
          (Animation|Montage|PlayMontage (Variables|Character|GetMesh) (Variables|/Game/StealthGameAIKit/Weapons/Base/BP_BaseWeapon.BP_BaseWeapon_C|GetReloadMontage (Variables|Weapon|GetCurrentWeapon))
            (:then
              (Audio|PlaySound2D "/Game/StealthGameAIKit/SFX/Reload/gunreload.gunreload" 1.0 1.0 0.0 0 0))
            (:OnCompleted
              (Default|CallOnEndReloaded :!label _label_2)
              (Variables|Weapon|SetbReloading false)
              (goto _label Reset))))))
    (:Is%20Not%20Valid
      (goto _label_2))))

(event Custom|WasSeen
  (params (Instigator :type BP%20Base%20Character%20Object%20Reference))
  ;[1 1 1] Override Events
)

(event Custom|Dead
  (params (BoneName :type Name) (ShotFromDirection :type Vector))
  (bind _self self)
  (bind _self_2 self)
  (bind _returnvalue (Pawn|GetController _self_2))
  ;[1 1 1] Dead
  (if (or (== _self "/Game/StealthGameAIKit/Characters/GuardAI/BP_Guard.BP_Guard") (== _self "/Game/StealthGameAIKit/Characters/AlarmGuard/BP_AlarmGuard.BP_AlarmGuard"))
    (AI|Logic|StopLogic (Variables|/Script/AIModule.AIController|GetBrainComponent (AI|GetAIController _self)) ""))
  (Input|DisableInput 0)
  (Utilities|IsValid _returnvalue
    (:Is%20Valid
      (Pawn|UnPossess _returnvalue))
    (:Is%20Not%20Valid
      _))
  (Pawn|Components|CharacterMovement|SetMovementMode (Variables|Character|GetCharacterMovement _self_2) "MOVE_None" 0)
  (CallFunction|RagdollActivated)
  (Class|SkeletalMeshComponent|AddImpulsetoAllBodiesBelow (Variables|Character|GetMesh) (* ShotFromDirection 0.0) BoneName false true)
  (Actor|SetLifeSpan 5.0))

(event Custom|OnGunFire
  ;[1 1 1] Override Events
)

(event Custom|Ragdoll%20Activated
  ;[1 1 1] Ragdoll
  (Utilities|FlowControl|Sequence
    (:then_0
      (bind _returnvalue (Utilities|Time|SetTimerbyEvent (delegate Custom|UpdateCollisionTransform) 0.1 true))
      (Utilities|FlowControl|Delay 3.0)
      (Utilities|Time|ClearandInvalidateTimerbyHandle _returnvalue))
    (:then_1
      (Components|Capsule|SetCapsuleHalfHeight (Variables|Collision|GetCapsuleComponent) 25.0 true)
      (Collision|SetCollisionEnabled (Variables|Collision|GetCapsuleComponent) "NoCollision")
      (Class|SkeletalMeshComponent|SetAllBodiesBelowSimulatePhysics (Variables|Character|GetMesh) (Utilities|FocusBoneName) true true)
      (Collision|SetCollisionProfileName (Variables|Character|GetMesh) "Ragdoll" true :!class /Script/Engine.PrimitiveComponent))))

(event Custom|UpdateCollisionTransform
  (bind _mesh (Variables|Character|GetMesh))
  (bind _returnvalue (Transformation|GetSocketTransform _mesh "spine_02" "RTS_World"))
  ;[1 1 1] Update Collision Transform
  (Transformation|SetWorldTransform (Variables|Collision|GetCapsuleComponent) (Math|Transform|MakeTransform (.location _returnvalue) (.rotation _returnvalue) "1,1,1") false false))

(event Custom|Begin%20Aim
  ;[1 1 1] Aim Events
  (Variables|Weapon|SetbAiming true)
  (Default|CallOnBeginAim))

(event Custom|End%20Aim
  ;[1 1 1] Aim Events
  (Variables|Weapon|SetbAiming false)
  (Default|CallOnEndAim))

(event Custom|TakeDamage
  (params (HitInfor :type Hit%20Result%20Structure))
  ;[1 1 1] Override Events
)

(event EventBeginPlay
  ;[1 1 1] Begin Play
  (Variables|Status|SetHealth (Variables|Config|Status|GetMaxHealth))
  (Initialize|SpawningWeapon)
  (EventDispatchers|AssignOnNeedReload (Variables|Weapon|GetWeaponInventory) (EventDispatchers|CreateEvent :!event Custom|ReloadWeapon))
  (EventDispatchers|BindEventtoOnFire (Variables|Weapon|GetWeaponInventory) (EventDispatchers|CreateEvent :!event Custom|OnGunFire)))

(event Game|Damage|EventPointDamage
  (params (Damage :type Float%20%28single-precision%29) (DamageType :type Damage%20Type%20Object%20Reference) (HitLocation :type Vector :default "0, 0, 0") (HitNormal :type Vector :default "0, 0, 0") (HitComponent :type Primitive%20Component%20Object%20Reference) (BoneName :type Name :default "None") (ShotFromDirection :type Vector :default "0, 0, 0") (InstigatedBy :type Controller%20Object%20Reference) (DamageCauser :type Actor%20Object%20Reference) (HitInfo :type Hit%20Result%20Structure%20%28by%20ref%29))
  ;[1 1 1] Damage
  (bind _output_get (Variables|Status|SetHealth (Common|CalcApplyDamageHealth Damage BoneName)))
  (Default|CallOnUpdateHealth _output_get (Variables|Config|Status|GetMaxHealth))
  (if (Status|IsDead)
    (CallFunction|Dead BoneName ShotFromDirection)
    (else
      (CallFunction|TakeDamage HitInfo)
      (CallFunction|PlayGruntSound))))

(event Input|KeyboardEvents|V
  (params (Key :type Key%20Structure :default "None"))
  ;[1 1 1] Save
  (:Pressed
    (bind _returnvalue (SaveGame|CreateSaveGameObject "/Game/StealthGameAIKit/SaveGame/BP_SaveGame.BP_SaveGame_C"))
    (Variables|/Game/StealthGameAIKit/SaveGame/BP_SaveGame.BP_SaveGame_C|SetCurrentHealth _returnvalue (Variables|Status|GetHealth))
    (for _array_element (Variables|Weapon|GetWeaponInventory)
      (Utilities|Map|Add (Variables|/Game/StealthGameAIKit/SaveGame/BP_SaveGame.BP_SaveGame_C|GetWeaponData _returnvalue) (.AsBP%20Base%20Weapon (Utilities|Casting|CastToBP_BaseWeaponClass (.WeaponClass (Utilities|Struct|BreakFWeaponData (Variables|/Game/StealthGameAIKit/Weapons/Base/BP_BaseWeapon.BP_BaseWeapon_C|GetWeaponData _array_element))))) (Variables|/Game/StealthGameAIKit/Weapons/Base/BP_BaseWeapon.BP_BaseWeapon_C|GetWeaponData _array_element))
      (bind _output_get (Variables|SaveGameProperties|SetActorLocation (Transformation|GetActorTransform self)))
      (Variables|/Game/StealthGameAIKit/SaveGame/BP_SaveGame.BP_SaveGame_C|SetActorCurrentLocation _returnvalue _output_get)
      ;;[1 1 1] Setting guardInfo
      (bind _outactors (Actor|GetAllActorsOfClass "/Game/StealthGameAIKit/Characters/GuardAI/BP_Guard.BP_Guard_C"))
      (for _array_element_2 _outactors
        (Utilities|Array|Add (Variables|SaveGameProperties|GetGuardInfo) (Utilities|Struct|MakeGuardInfoStruct (Variables|/Game/StealthGameAIKit/Characters/GuardAI/BP_Guard.BP_Guard_C|GetIsGuardDead _array_element_2) _array_element_2 (Transformation|GetActorTransform _array_element_2))))
      (Variables|/Game/StealthGameAIKit/SaveGame/BP_SaveGame.BP_SaveGame_C|SetSavedGuardData _returnvalue (Variables|SaveGameProperties|GetGuardInfo))
      (bind _outactors_2 (Actor|GetAllActorsOfClass "/Game/StealthGameAIKit/Placeables/Pickups/Collectible/BP_Key.BP_Key_C"))
      (for _array_element_3 _outactors_2
        (if (Variables|/Game/StealthGameAIKit/Placeables/Pickups/Base/BP_BasePickup.BP_BasePickup_C|GetCollected _array_element_3)
          (Utilities|Array|Add (Variables|SaveGameProperties|GetCollectedObject) _array_element_3)))
      (Variables|/Game/StealthGameAIKit/SaveGame/BP_SaveGame.BP_SaveGame_C|SetSavedCollectibls _returnvalue (Variables|SaveGameProperties|GetCollectedObject))
      (SaveGame|SaveGametoSlot _returnvalue "SaveSlot"))))

(event Input|KeyboardEvents|L
  (params (Key :type Key%20Structure :default "None"))
  (bind _currentweapon (Variables|Weapon|GetCurrentWeapon))
  ;[1 1 1] Load
  (:Pressed
    ;;[1 1 1] Load From slot
    (bind _returnvalue (SaveGame|LoadGamefromSlot "SaveSlot"))
    (bind _asbp_save_game (Utilities|Casting|CastToBP_SaveGame _returnvalue))
    (Development|PrintString (Utilities|String|ToString(Integer) (Utilities|Array|Length (Variables|/Game/StealthGameAIKit/SaveGame/BP_SaveGame.BP_SaveGame_C|GetSavedCollectibls _asbp_save_game))))
    ;;[1 1 1] change health
    (bind _output_get (Variables|Status|SetHealth (Variables|/Game/StealthGameAIKit/SaveGame/BP_SaveGame.BP_SaveGame_C|GetCurrentHealth _asbp_save_game)))
    (Default|CallOnUpdateHealth _output_get 1e+01)
    ;;[1 1 1] change the players weapon data
    (for _array_element (Variables|Weapon|GetWeaponInventory)
      (Variables|/Game/StealthGameAIKit/Weapons/Base/BP_BaseWeapon.BP_BaseWeapon_C|SetWeaponData _array_element (.Value (Utilities|Map|Find (Variables|/Game/StealthGameAIKit/SaveGame/BP_SaveGame.BP_SaveGame_C|GetWeaponData _asbp_save_game) (Utilities|GetClass _array_element))))
      ;;[1 1 1] Change location
      (bind _output_get_2 (Variables|SaveGameProperties|SetActorLocation (Variables|/Game/StealthGameAIKit/SaveGame/BP_SaveGame.BP_SaveGame_C|GetActorCurrentLocation _asbp_save_game)))
      (Transformation|SetActorLocationAndRotation self (.location _output_get_2) (.rotation _output_get_2))
      ;;[1 1 1] Change the guards location
      (for _array_element_2 (Variables|/Game/StealthGameAIKit/SaveGame/BP_SaveGame.BP_SaveGame_C|GetSavedGuardData _asbp_save_game)
        (Transformation|SetActorTransform (.id _array_element_2) (.position _array_element_2))
        ;;[1 1 1] Call Dead if the guard is dead
        (if (.isdead _array_element_2)
          (CallFunction|Dead (.id _array_element_2) "None" "0, 0, 0")))
      (for _array_element_3 (Variables|/Game/StealthGameAIKit/SaveGame/BP_SaveGame.BP_SaveGame_C|GetSavedCollectibls _asbp_save_game)
        (Default|ApplyPickupEffects _array_element_3)))
    (Default|CallOnUpdateWidget _currentweapon (Variables|/Game/StealthGameAIKit/Weapons/Base/BP_BaseWeapon.BP_BaseWeapon_C|GetWeaponData _currentweapon))))

(fn ConstructionScript)

(fn IsDead
  (return (<= (Variables|Status|GetHealth) 0.0)))

(fn CalcApplyDamageHealth
  (params (DamageAmount :type Float%20%28single-precision%29) (BoneName :type Name))
  (bind _returnvalue (Utilities|Name|Equal(Name) BoneName "head"))
  (bind _returnvalue_2 (Utilities|Name|Equal(Name) BoneName "neck_01"))
  (bind _returnvalue_3 (or _returnvalue _returnvalue_2))
  (if _returnvalue_3
    (CallFunction|Dead BoneName "0, 0, 0")
    (else
      (return (|(Max(({DD5E3E14-4271-F474-7B2D-5BA68F3FD6F1}-(Coefficient*Damage)),0)) DamageAmount (Math|Float|SelectFloat 1e+03 1.0 _returnvalue_3))))))

(fn SpawningWeapon
  (bind _self self)
  (for _array_element (Variables|Config|Weapon|GetDefaultWeaponInventory)
    (bind _returnvalue (Game|SpawnActorfromClass _array_element (Transformation|GetActorTransform) "AlwaysSpawn" _self _self))
    (Utilities|Array|AddUnique (Variables|Weapon|GetWeaponInventory) (.AsBP%20Base%20Weapon (Utilities|Casting|CastToBP_BaseWeapon _returnvalue))))
  (return))

(fn IsAlive
  (return (not (Status|IsDead))))

(fn PlayGruntSound
  (Audio|PlaySoundatLocation (.OutItem (Utilities|Array|Random (Variables|Default|GetGruntSounds))) (Transformation|GetActorLocation self) "0, 0, 0" 1.0 1.0 0.0 0 0 0))

(fn PlayDeathSound
  (params (Location :type Vector))
  (Audio|PlaySoundatLocation (.OutItem (Utilities|Array|Random (Variables|Default|GetDeathSounds))) Location "0, 0, 0" 1.0 1.0 0.0 0 0 0))