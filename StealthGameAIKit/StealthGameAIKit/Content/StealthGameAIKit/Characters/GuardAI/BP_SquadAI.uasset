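; BP_SquadAI relays squad alerts between stealth-game guards: enemy found, enemy dead, enemy lost and ally body found.
; Each notify event sphere-overlaps BP_Guard pawns around the instigator, excluding it, and calls the matching Received function on each living ally's AIC_Guard controller.
; Lost-enemy and dead-body alerts give each ally its own random reachable point near the reported position, spreading out the responders.
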(event Custom|NotifyFindEnemy
  (params (InstigatorPawn :type BP%20Guard%20Object%20Reference) (InstigatorController :type AIC%20Guard%20Object%20Reference) (NotifyRadius :type Float%20%28single-precision%29) (EnemyActor :type BP%20Base%20Character%20Object%20Reference))
  ;[1 1 1] Notify nearby allies that they have found an enemy
  (bind _return (CallFunction|SearchNearbyAllies (Transformation|GetActorLocation InstigatorPawn) NotifyRadius InstigatorPawn))
  (for _array_element _return
    (if (Default|IsAlive _array_element)
      (Default|ReceivedFoundEnemy (.AsAIC%20Guard (Utilities|Casting|CastToAIC_Guard (AI|GetAIController _array_element))) EnemyActor))))

(event Custom|NotifyEnemyIsDead
  (params (InstigatorPawn :type BP%20Guard%20Object%20Reference) (InstigatorController :type AIC%20Guard%20Object%20Reference) (NotifyRadius :type Float%20%28single-precision%29))
  (bind _return (CallFunction|SearchNearbyAllies (Transformation|GetActorLocation InstigatorPawn) NotifyRadius InstigatorPawn))
  (for _array_element _return
    (if (Default|IsAlive _array_element)
      (Default|ReceivedEnemyIsDead (.AsAIC%20Guard (Utilities|Casting|CastToAIC_Guard (AI|GetAIController _array_element)))))))

(event Custom|NotifyLostEnemy
  (params (InstigatorPawn :type BP%20Guard%20Object%20Reference) (InstigatorController :type AIC%20Guard%20Object%20Reference) (NotifyRadius :type Float%20%28single-precision%29) (CenterPosition :type Vector))
  (bind _return (CallFunction|SearchNearbyAllies (Transformation|GetActorLocation InstigatorPawn) NotifyRadius InstigatorPawn))
  (for _array_element _return
    (if (Default|IsAlive _array_element)
      (Default|ReceivedLostEnemy (.AsAIC%20Guard (Utilities|Casting|CastToAIC_Guard (AI|GetAIController _array_element))) (.RandomLocation (AI|Navigation|GetRandomReachablePointinRadius CenterPosition 2.5e+02 0 0))))))

(event Custom|NotifyFoundAllyDeadbody
  (params (InstigatorPawn :type BP%20Guard%20Object%20Reference) (InstigatorController :type AIC%20Guard%20Object%20Reference) (NotifyRadius :type Float%20%28single-precision%29) (CenterPosition :type Vector))
  (bind _return (CallFunction|SearchNearbyAllies (Transformation|GetActorLocation InstigatorPawn) NotifyRadius InstigatorPawn))
  (for _array_element _return
    (if (Default|IsAlive _array_element)
      (Default|ReceivedFindAllyDeadbody (.AsAIC%20Guard (Utilities|Casting|CastToAIC_Guard (AI|GetAIController _array_element))) (.RandomLocation (AI|Navigation|GetRandomReachablePointinRadius CenterPosition 2.5e+02 0 0))))))

(fn ConstructionScript)

(fn SearchNearbyAllies
  (params (Center :type Vector) (SearchRadius :type Float%20%28single-precision%29) (Instigator :type BP%20Guard%20Object%20Reference))
  (bind _outactors (Collision|SphereOverlapActors Center SearchRadius (Utilities|Array|MakeArray "ObjectTypeQuery3") "/Game/StealthGameAIKit/Characters/GuardAI/BP_Guard.BP_Guard_C" (Utilities|Array|MakeArray Instigator)))
  (for _array_element _outactors
    (Utilities|Array|Add (LocalVariables|GetNearbyAllies) (.AsBP%20Guard (Utilities|Casting|CastToBP_Guard _array_element))))
  (return (LocalVariables|GetNearbyAllies)))