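; BP_Guard is the stealth AI guard character, driven by AIC_Guard and linked to a SquadAI.
; Patrol, Search and Attack states set speed, aim and body color, with spline, random or stationary patrol destinations.
; It fires at the controller's enemy, reports gunfire noise, and pauses AI logic to turn toward shots.
; Overlap boxes offer player takedowns and too-close detection, while widgets show sight, spot marker and reaction icons.
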(event OnComponentBeginOverlap(StealthBox)
  (params (OverlappedComponent :type Primitive%20Component%20Object%20Reference) (OtherActor :type Actor%20Object%20Reference) (OtherComp :type Primitive%20Component%20Object%20Reference) (OtherBodyIndex :type Integer) (bFromSweep :type Boolean) (SweepResult :type Hit%20Result%20Structure%20%28by%20ref%29))
  ;[1 1 1] Add widgets on overlap
  (if (not (Variables|Default|GetIsGuardDead))
    (bind _asbp_player (Utilities|Casting|CastToBP_Player OtherActor))
    (Utilities|IsValid (Variables|/Game/StealthGameAIKit/Characters/Player/BP_Player.BP_Player_C|GetPossibleVictim _asbp_player)
      (:Is%20Not%20Valid
        (Variables|/Game/StealthGameAIKit/Characters/Player/BP_Player.BP_Player_C|SetPossibleVictim _asbp_player self)
        (bind _returnvalue (UserInterface|CreateWidget "/Game/StealthGameAIKit/UserInterface/TakedownWidget.TakedownWidget_C"))
        (bind _output_get (Variables|Default|SetTakedownWidget _returnvalue))
        (UserInterface|Viewport|AddtoViewport _output_get 0)
        (Variables|/Game/StealthGameAIKit/Characters/Player/BP_Player.BP_Player_C|SetTakedownWidget _asbp_player (Variables|Default|GetTakedownWidget))))))

(event OnComponentEndOverlap(StealthBox)
  (params (OverlappedComponent :type Primitive%20Component%20Object%20Reference) (OtherActor :type Actor%20Object%20Reference) (OtherComp :type Primitive%20Component%20Object%20Reference) (OtherBodyIndex :type Integer))
  (bind _takedownwidget (Variables|Default|GetTakedownWidget))
  ;[1 1 1] Add widgets on overlap
  (bind _asbp_player (Utilities|Casting|CastToBP_Player OtherActor))
  (Variables|/Game/StealthGameAIKit/Characters/Player/BP_Player.BP_Player_C|SetPossibleVictim _asbp_player 0)
  (Utilities|IsValid _takedownwidget
    (:Is%20Valid
      (Widget|RemovefromParent _takedownwidget))))

(event OnComponentBeginOverlap(Box)
  (params (OverlappedComponent :type Primitive%20Component%20Object%20Reference) (OtherActor :type Actor%20Object%20Reference) (OtherComp :type Primitive%20Component%20Object%20Reference) (OtherBodyIndex :type Integer) (bFromSweep :type Boolean) (SweepResult :type Hit%20Result%20Structure%20%28by%20ref%29))
  (if (== OtherActor (Game|Player|GetPlayerPawn 0))
    (Utilities|Casting|CastToAIC_Guard (AI|GetAIController (Components|GetOwner)))
    (Default|TooClose (Variables|Default|GetWBPSightDetection))))

(event Custom|ChangeState
  (params (NewState :type EGuardState%20Enum :default "NewEnumerator0"))
  ;[1 1 1] Comment
  (bind _output_get (Variables|Default|SetGuardState NewState))
  (switch Utilities|FlowControl|Switch|SwitchonEGuardState _output_get
    (:NewEnumerator0
      (Character|UnCrouch)
      (Variables|Default|SetbAiming false)
      (Variables|/Script/Engine.CharacterMovementComponent|SetMaxWalkSpeed (Variables|Character|GetCharacterMovement) (Variables|Status|GetPatrolWalkSpeed))
      (Rendering|Material|SetVectorParameterValue (Variables|Materials|GetBodyMatInstance) "BodyColor" "(R=0.450980,G=0.403922,B=0.360784,A=0.000000)" :!class /Script/Engine.MaterialInstanceDynamic))
    (:NewEnumerator1
      (Variables|Default|SetbAiming true)
      (Variables|/Script/Engine.CharacterMovementComponent|SetMaxWalkSpeed (Variables|Character|GetCharacterMovement) (Variables|Status|GetSearchWalkSpeed))
      (Rendering|Material|SetVectorParameterValue (Variables|Materials|GetBodyMatInstance) "BodyColor" "(R=1.000000,G=0.305000,B=0.000000,A=0.000000)" :!class /Script/Engine.MaterialInstanceDynamic))
    (:NewEnumerator2
      (Default|TargetLost (Variables|Default|GetWBPSightDetection))
      (Variables|Default|SetbAiming true)
      (Variables|/Script/Engine.CharacterMovementComponent|SetMaxWalkSpeed (Variables|Character|GetCharacterMovement) (Variables|Status|GetAttackWalkSpeed))
      (Rendering|Material|SetVectorParameterValue (Variables|Materials|GetBodyMatInstance) "BodyColor" "(R=1.000000,G=0.000000,B=0.000000,A=0.000000)" :!class /Script/Engine.MaterialInstanceDynamic)))
  (CallFunction|ReadyShowBillboard))

(event Custom|Attack
  (bind (_return _bsuccess) (Getter|GetEnemeyCharacter))
  ;[1 1 1] Fire Weapon
  (Utilities|IsValid (Variables|Default|GetCurrentWeapon)
    (:Is%20Valid
      (if _bsuccess
        (Default|Fire (Variables|Default|GetCurrentWeapon) (Math|MuzzletoMeshSocket _return "spine_02") 0.0 "BP_Guard_C")))))

(event Custom|LookAtTarget
  (params (NewParam :type Vector))
  ;[1 1 1] Look at Target
  (bind _alpha (Timeline|TimelineEaseAlpha PlayFromStart)
    (:Update
      (Transformation|SetActorRotation (Math|Rotator|MakeRotator 0.0 0.0 (.yaw (Math|Interpolation|Ease "CircularOut" _alpha (Transformation|GetActorRotation) (Math|Rotator|FindLookatRotation (Transformation|GetActorLocation) NewParam) true))))
      (Utilities|FlowControl|Delay 5.0))))

(event Custom|Unmarked%20Indicator
  ;[1 1 1] Show & Hidden Mark Indicator
  (Rendering|SetVisibility (Variables|Default|GetSpotMarker) false false))

(event Custom|Mark%20Indicator
  ;[1 1 1] Show & Hidden Mark Indicator
  (Rendering|SetVisibility (Variables|Default|GetSpotMarker) true false))

(event Custom|ShowReactionBillboard
  (params (Exclamation :type Boolean))
  ;[1 1 1] Show Reaction Billboard
  (Utilities|FlowControl|DoOnce false
    (:Completed
      (Default|PlayBeginAnim (.AsWBP%20Reaction%20Billboard (Utilities|Casting|CastToWBP_ReactionBillboard (UserInterface|GetUserWidgetObject (Variables|Default|GetReactionIcon)))) Exclamation))))

(event Custom|ReadyShowBillboard
  ;[1 1 1] Show Reaction Billboard
  (Utilities|FlowControl|DoOnce false) ; enters at Reset
)

(event Game|Damage|EventPointDamage
  (params (Damage :type Float%20%28single-precision%29) (DamageType :type Damage%20Type%20Object%20Reference) (HitLocation :type Vector :default "0, 0, 0") (HitNormal :type Vector :default "0, 0, 0") (HitComponent :type Primitive%20Component%20Object%20Reference) (BoneName :type Name :default "None") (ShotFromDirection :type Vector :default "0, 0, 0") (InstigatedBy :type Controller%20Object%20Reference) (DamageCauser :type Actor%20Object%20Reference) (HitInfo :type Hit%20Result%20Structure%20%28by%20ref%29))
  (bind _self self)
  (bind _returnvalue (AI|GetAIController _self))
  ;[1 1 1] Take Point Damage
  (|CallParentFunction Damage DamageType HitLocation HitNormal HitComponent BoneName ShotFromDirection InstigatedBy DamageCauser HitInfo)
  (if (CallFunction|IsAlive)
    (Utilities|FlowControl|Sequence
      (:then_0
        (CallFunction|LookatTarget (+ (Transformation|GetActorLocation) (* (Math|Vector|NegateVector ShotFromDirection) 1e+02)))
        (AI|Logic|StopLogic (Variables|/Script/AIModule.AIController|GetBrainComponent (AI|GetAIController self)) ""))
      (:then_1
        (Utilities|FlowControl|Delay (Components|Timeline|GetTimelineLength (Variables|Default|GetTimelineEaseAlpha)))
        (Utilities|IsValid _returnvalue
          (:Is%20Valid
            (Class|BrainComponent|RestartLogic (Variables|/Script/AIModule.AIController|GetBrainComponent _returnvalue))))))))

(event EventOnGunFire
  ;[1 1 1] On Fire
  (Class|AISenseHearing|ReportNoiseEvent (Transformation|GetActorLocation) 1.0 self 1.2e+03 "None"))

(event EventBeginPlay
  ;[1 1 1] Begin Play
  (|CallParentFunction)
  (Utilities|FlowControl|Sequence
    (:then_0
      (bind _aswbp_sight_detection (Utilities|Casting|CastToWBP_SightDetection (UserInterface|GetUserWidgetObject (Variables|Default|GetWidget))))
      (Variables|/Game/StealthGameAIKit/Characters/GuardAI/WBP_SightDetection.WBP_SightDetection_C|SetPawnOwner _aswbp_sight_detection self)
      (bind _output_get (Variables|Default|SetWBPSightDetection _aswbp_sight_detection))
      (bind _asaic_guard (Utilities|Casting|CastToAIC_Guard (AI|GetAIController self)))
      (Variables|/Game/StealthGameAIKit/Characters/GuardAI/AIC_Guard.AIC_Guard_C|SetWidget _asaic_guard _output_get)
      (Utilities|IsValid (Variables|Config|Squad|GetSquadAI)
        (:Is%20Valid
          (bind _returnvalue (Rendering|Material|CreateDynamicMaterialInstance (Variables|Character|GetMesh) 0 (Rendering|Material|GetMaterial (Variables|Character|GetMesh) 0) "None" :!class /Script/Engine.PrimitiveComponent))
          (Variables|Materials|SetBodyMatInstance _returnvalue)
          (CallFunction|ChangeState "NewEnumerator0")
          (CallFunction|EquipWeapon))
        (:Is%20Not%20Valid
          (Development|PrintString "ERROR : SquadAI is Not Invalid" true true "(R=1.000000,G=0.000000,B=0.000000,A=1.000000)"))))
    (:then_1
      (Variables|/Game/StealthGameAIKit/Characters/GuardAI/WBP_SpotMarker.WBP_SpotMarker_C|SetOwnerPawn (.AsWBP%20Spot%20Marker (Utilities|Casting|CastToWBP_SpotMarker (UserInterface|GetUserWidgetObject (Variables|Default|GetSpotMarker)))) self)
      (Rendering|SetVisibility (Variables|Default|GetSpotMarker) false false)
      (Variables|Patrol|SetPatrolStartLocation (Transformation|GetActorLocation))
      (Variables|Patrol|SetPatrolStartRotation (Transformation|GetActorRotation))
      (Variables|Patrol|SetCurrentWaypointIndex (Variables|Config|PatrolParams|SplineBased|GetBeginPatrolWaypointIndex)))))

(event EventDead
  (params (BoneName :type Name :default "None") (ShotFromDirection :type Vector :default "0, 0, 0"))
  (bind _widget (Variables|Default|GetWidget))
  (bind _reactionicon (Variables|Default|GetReactionIcon))
  ;[1 1 1] Dead
  (|CallParentFunction BoneName ShotFromDirection)
  (CallFunction|UnmarkedIndicator)
  (Class|Pawn|DetachfromControllerPendingDestroy)
  (Variables|Default|SetIsGuardDead true)
  (Utilities|IsValid _widget
    (:Is%20Valid
      (Components|DestroyComponent _widget)
      (Utilities|IsValid _reactionicon
        (:Is%20Valid
          (Components|DestroyComponent _reactionicon))))))

(event EventPossessed
  (params (NewController :type Controller%20Object%20Reference))
  ;[1 1 1] Possessed
  (bind _asaic_guard (Utilities|Casting|CastToAIC_Guard NewController))
  (Variables|/Game/StealthGameAIKit/Characters/GuardAI/AIC_Guard.AIC_Guard_C|SetSquadAI _asaic_guard (Variables|Config|Squad|GetSquadAI)))

(event Game|Damage|EventAnyDamage
  (params (Damage :type Float%20%28single-precision%29) (DamageType :type Damage%20Type%20Object%20Reference) (InstigatedBy :type Controller%20Object%20Reference) (DamageCauser :type Actor%20Object%20Reference))
  ;[1 1 1] Any Damage
  (|CallParentFunction Damage DamageType "0, 0, 0" "0, 0, 0" 0 "None" "0, 0, 0" InstigatedBy DamageCauser (Collision|MakeHitResult false false 0.0 0.0 "0, 0, 0" "0, 0, 0" "0,0,1" "0,0,1" 0 0)))

(fn ConstructionScript
  (switch Utilities|FlowControl|Switch|SwitchonEPatrolType (Variables|Config|Patrol|GetPatrolType)
    (:NewEnumerator1
      (Rendering|Debug|DrawDebugCircle (Transformation|GetActorLocation) (Variables|Config|PatrolParams|Random|GetRandomPatrolRange) 36 "(R=1.000000,G=1.000000,B=1.000000,A=1.000000)" 1.0 1e+01 "1.000000,0.000000,0.000000" "0.000000,1.000000,0.000000") ; Highlighting Wander Radius
    )))

(fn GetEnemeyCharacter
  (bind _self self)
  (bind _returnvalue (AI|GetAIController _self))
  (bind _asaic_guard (Utilities|Casting|CastToAIC_Guard _returnvalue))
  (bind (_enemyref _success) (Default|GetEnemyValue _asaic_guard))
  (return _enemyref _success))

(fn NextPatrolDestinationandRotation
  (Utilities|FlowControl|Sequence
    (:then_0
      (switch Utilities|FlowControl|Switch|SwitchonEPatrolType (Variables|Config|Patrol|GetPatrolType)
        (:NewEnumerator0
          (LocalVariables|SetLocalDestination (.Location (Default|GetNextDestination (Variables|Config|PatrolParams|SplineBased|GetPatrolSpline) (Variables|Patrol|GetCurrentWaypointIndex) (Variables|Patrol|GetbPatrolDirectionForward))))
          (Variables|Patrol|SetCurrentWaypointIndex (.NextWaypointIndex (Default|GetNextDestination (Variables|Config|PatrolParams|SplineBased|GetPatrolSpline) (Variables|Patrol|GetCurrentWaypointIndex) (Variables|Patrol|GetbPatrolDirectionForward))))
          (Variables|Patrol|SetbPatrolDirectionForward (.NextPatrolDirection (Default|GetNextDestination (Variables|Config|PatrolParams|SplineBased|GetPatrolSpline) (Variables|Patrol|GetCurrentWaypointIndex) (Variables|Patrol|GetbPatrolDirectionForward))))
          (LocalVariables|SetLocalRotate (Math|Rotator|MakeRotator 0.0 0.0 (.yaw (Math|Rotator|FindLookatRotation (Transformation|GetActorLocation) (LocalVariables|GetLocalDestination))))))
        (:NewEnumerator1
          (LocalVariables|SetLocalDestination (.RandomLocation (AI|Navigation|GetRandomReachablePointinRadius (Variables|Patrol|GetPatrolStartLocation) (Variables|Config|PatrolParams|Random|GetRandomPatrolRange) 0 0)))
          (LocalVariables|SetLocalRotate (Math|Rotator|MakeRotator 0.0 0.0 (.yaw (Math|Rotator|FindLookatRotation (Transformation|GetActorLocation) (LocalVariables|GetLocalDestination))))))
        (:NewEnumerator2
          (LocalVariables|SetLocalDestination (Variables|Patrol|GetPatrolStartLocation))
          (LocalVariables|SetLocalRotate (Variables|Patrol|GetPatrolStartRotation)))))
    (:then_1
      (return (LocalVariables|GetLocalDestination) (LocalVariables|GetLocalRotate)))))

(fn MuzzletoMeshSocket
  (params (MeshOwner :type Character%20Object%20Reference) (SocketName :type Name))
  (return (Math|Vector|Normalize (- (Transformation|GetSocketLocation (Variables|/Script/Engine.Character|GetMesh MeshOwner) SocketName) (Default|GetMuzzleLocation (Variables|Default|GetCurrentWeapon))))))

(fn IsNotInvestigated
  (return (not (Variables|Status|GetbInvestigated))))