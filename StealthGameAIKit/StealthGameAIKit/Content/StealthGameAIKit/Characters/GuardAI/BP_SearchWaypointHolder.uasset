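; BP_SearchWaypointHolder is a guard AI helper actor that lays out a square grid of search waypoints around its location.
; On BeginPlay, GenerateWaypoint derives the grid from half-size and spacing, projecting each point onto the navmesh and spawning a BP_SearchWaypoint only where projection succeeds.
; Spawned waypoints are tracked in an array and destroyed with the holder.
; A separate SpawnGridWaypoint function places one row/column point but is not called here.
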(event EventBeginPlay
  (CallFunction|GenerateWaypoint))

(event EventDestroyed
  (Actor|DestroyActor (Variables|Default|GetWaypoints))
  (Utilities|Array|Clear (Variables|Default|GetWaypoints)))

(fn ConstructionScript)

(fn SpawnGridWaypoint
  (params (Row :type Integer) (Col :type Integer))
  (Utilities|FlowControl|Sequence
    (:then_0
      (LocalVariables|SetLocationX (|((({754A831C-4DFE-1CCE-AFD5-AAA3E3B2ED68}*0.500000)*RowCol)-{754A831C-4DFE-1CCE-AFD5-AAA3E3B2ED68}) Row))
      (LocalVariables|SetLocationY (|((({754A831C-4DFE-1CCE-AFD5-AAA3E3B2ED68}*0.500000)*RowCol)-{754A831C-4DFE-1CCE-AFD5-AAA3E3B2ED68}) Col)))
    (:then_1
      (if (.ReturnValue (AI|Navigation|ProjectPointtoNavigation (+ (Transformation|GetActorLocation) (Math|Vector|MakeVector (LocalVariables|GetLocationX) (LocalVariables|GetLocationY) 0.0)) 0 0 "25.000000,25.000000,500.000000"))
        (bind _returnvalue (Game|SpawnActorfromClass "/Game/StealthGameAIKit/Characters/GuardAI/BP_SearchWaypoint.BP_SearchWaypoint_C" (Math|Transform|MakeTransform (.ProjectedLocation (AI|Navigation|ProjectPointtoNavigation (+ (Transformation|GetActorLocation) (Math|Vector|MakeVector (LocalVariables|GetLocationX) (LocalVariables|GetLocationY) 0.0)) 0 0 "25.000000,25.000000,500.000000")) "0, 0, 0" "1,1,1") "AdjustIfPossibleButAlwaysSpawn" 0 (Variables|Actor|GetInstigator)))
        (Utilities|Array|Add (Variables|Default|GetWaypoints) _returnvalue)
        (return)
        (else
          (return))))))

(fn GenerateWaypoint
  (bind _output_get (LocalVariables|SetItemCount (Math|Float|Truncate (|((({FC2962F2-4179-CFE3-1B90-1EAF14893102}*2.000000)/{DBA5C2FD-4A2B-A998-4086-5AA289E64101})+1)))))
  (LocalVariables|SetItemCountHalf (/ _output_get 2))
  (for _index (range 0 (- (LocalVariables|GetItemCount) 1)) ; X
    (LocalVariables|SetX _index)
    (for _index_2 (range 0 (- (LocalVariables|GetItemCount) 1)) ; Y
      (LocalVariables|SetY _index_2)
      (if (.ReturnValue (AI|Navigation|ProjectPointtoNavigation (- (Transformation|GetActorLocation) (Math|Vector|MakeVector (|({DBA5C2FD-4A2B-A998-4086-5AA289E64101}*(Num-{DB5EA417-4AB5-F956-C08E-CA925B93B47A})) (LocalVariables|GetX)) (|({DBA5C2FD-4A2B-A998-4086-5AA289E64101}*(Num-{DB5EA417-4AB5-F956-C08E-CA925B93B47A})) (LocalVariables|GetY)) 0.0)) 0 0 "25.000000,25.000000,500.000000"))
        (bind _returnvalue (Game|SpawnActorfromClass "/Game/StealthGameAIKit/Characters/GuardAI/BP_SearchWaypoint.BP_SearchWaypoint_C" (Math|Transform|MakeTransform (.ProjectedLocation (AI|Navigation|ProjectPointtoNavigation (- (Transformation|GetActorLocation) (Math|Vector|MakeVector (|({DBA5C2FD-4A2B-A998-4086-5AA289E64101}*(Num-{DB5EA417-4AB5-F956-C08E-CA925B93B47A})) (LocalVariables|GetX)) (|({DBA5C2FD-4A2B-A998-4086-5AA289E64101}*(Num-{DB5EA417-4AB5-F956-C08E-CA925B93B47A})) (LocalVariables|GetY)) 0.0)) 0 0 "25.000000,25.000000,500.000000")) "0, 0, 0" "1,1,1") "AdjustIfPossibleButAlwaysSpawn" 0 (Variables|Actor|GetInstigator)))
        (Utilities|Array|Add (Variables|Default|GetWaypoints) _returnvalue))))
  (return))