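; BP_SearchWaypoint is a guard AI search point that records whether its instigating guard has visited it.
; Each tick it requires an unblocked Visibility trace to the guard and a squared-distance check against a fixed radius.
; When both pass, it sets Visited, turns its arrow red and disables its own tick.
; GetVisited exposes the flag to other logic.
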(event EventBeginPlay
  (Actor|Tick|SetActorTickEnabled true))

(event EventTick
  (params (DeltaSeconds :type Float%20%28single-precision%29))
  (if (and (CallFunction|CheckObstacleBetweenSelfandGuards) (CallFunction|IsClosetoGuardPawn 7.5e+02))
    (Variables|Default|SetbVisited true)
    (Actor|Tick|SetActorTickEnabled false)
    (Components|Arrow|SetArrowColor(LinearColor) (Variables|Default|GetArrow) "(R=1.000000,G=0.000000,B=0.000000,A=1.000000)")))

(fn ConstructionScript)

(fn IsClosetoGuardPawn
  (params (Threshold :type Float%20%28single-precision%29))
  (bind _instigator (Variables|Actor|GetInstigator))
  (LocalVariables|SetCloseDistanceSq (Math|Float|Power Threshold 2.0))
  (Utilities|IsValid _instigator
    (:Is%20Valid
      (LocalVariables|SetToGuardPawnDistSq (Class|KismetMathLibrary|VectorDistanceSquared (Transformation|GetActorLocation _instigator) (Transformation|GetActorLocation)))
      (return (< (LocalVariables|GetToGuardPawnDistSq) (LocalVariables|GetCloseDistanceSq))))))

(fn CheckObstacleBetweenSelfandGuards
  (bind _instigator (Variables|Actor|GetInstigator))
  (Utilities|IsValid _instigator
    (:Is%20Valid
      (bind _outhit (Collision|LineTraceByChannel (+ (Transformation|GetActorLocation) "0, 0,10.000000") (Transformation|GetActorLocation _instigator) "TraceTypeQuery1" false 0 "None" true "(R=1.000000,G=0.000000,B=0.000000,A=1.000000)" "(R=0.000000,G=1.000000,B=0.000000,A=1.000000)" 0.5))
      (return (not (.bblockinghit _outhit))))))

(fn GetVisited
  (return (Variables|Default|GetbVisited)))