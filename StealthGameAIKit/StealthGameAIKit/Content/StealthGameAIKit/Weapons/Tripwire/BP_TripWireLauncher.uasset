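; BP_TripWireLauncher is a weapon whose Fire event installs a BP_TripWire trap if ammo remains.
; Firing disables the owner pawn's input and plays an install montage, while a timeline drives an on-screen progress bar widget.
; A montage notify spawns the trip wire at the weapon mesh's transform, decrements ammo and updates the weapon widget.
; Montage completion restores input and removes the bar.
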(event EventBeginPlay
  (|CallParentFunction) ; This node is disabled and will not be called.\nDrag off pins to build functionality.
)

(event Collision|EventActorBeginOverlap
  (params (OtherActor :type Actor%20Object%20Reference)))

(event EventTick
  (params (DeltaSeconds :type Float%20%28single-precision%29)))

(event EventFire
  (params (Direction :type Vector :default "0, 0, 0") (RandomHalfAngle :type Float%20%28single-precision%29) (FilterClass :type BP%20Base%20Character%20Class%20Reference))
  (if (not (CallFunction|IsEmptyAmmo))
    (Input|DisableInput (Variables|Default|GetOwnerPawn) 0)
    (Animation|Montage|PlayMontage (Variables|/Script/Engine.Character|GetMesh (Variables|Default|GetOwnerPawn)) "/Game/Animations/Loot_Anim_Set/Animations/Loot_Corpse/InstallTrap_Montage.InstallTrap_Montage"
      (:then
        (bind _returnvalue (UserInterface|CreateWidget "/Game/StealthGameAIKit/progressbar/WB_Testbar.WB_Testbar_C"))
        (UserInterface|Viewport|AddtoViewport _returnvalue 0)
        (bind _percentage (Timeline|Timeline_0 PlayFromStart)
          (:Update
            (Default|SetPercent _returnvalue _percentage))))
      (:OnCompleted
        ;[1 1 1] spawn new trip wire + enable input
        (Input|EnableInput (Variables|Default|GetOwnerPawn) 0)
        (Widget|RemovefromParent _returnvalue))
      (:OnNotifyBegin
        (Game|SpawnActorfromClass "/Game/StealthGameAIKit/Weapons/Tripwire/BP_TripWire.BP_TripWire_C" (Transformation|GetWorldTransform (Variables|Default|GetWeaponSkeletalMesh)) "Undefined" 0 0)
        (Math|Integer|DecrementInt (.currentammo (Variables|Default|GetWeaponData))
          (:%20%20
            (Default|CallOnUpdateWidget (Variables|Default|GetWeaponData))))))))

(fn ConstructionScript
  (|CallParentFunction))