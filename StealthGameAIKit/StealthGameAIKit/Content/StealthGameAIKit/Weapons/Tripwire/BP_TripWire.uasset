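; BP_TripWire is a placeable tripwire that pairs with another and damages guards crossing the line between them.
; On BeginPlay it links to the closest unpaired tripwire within range and line of sight, becomes master and attaches its cable to the partner.
; Each tick only the master traces for pawns along the span, applying point damage whenever the hit is a BP_Guard.
; Both traces draw debug lines.
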(event EventBeginPlay
  (bind _pairedobject (CallFunction|CheckforPair))
  (if (Utilities|IsValid _pairedobject)
    (Variables|Default|SetMaster true)
    (bind _output_get (Variables|Default|Setpartner _pairedobject))
    (Variables|BP_TripWire_C|Setpartner _output_get self)
    (Class|CableComponent|SetAttachEndto (Variables|Default|GetCable) (Variables|Default|Getpartner) "None" "None")
    (Development|PrintString "Collied")))

(event EventTick
  (params (DeltaSeconds :type Float%20%28single-precision%29))
  (bind _partner (Variables|Default|Getpartner))
  (if (and (Utilities|IsValid _partner) (Variables|Default|GetMaster))
    (bind (_outhit _returnvalue) (Collision|LineTraceForObjects (+ (Transformation|GetActorLocation) "0, 0,20.000000") (+ (Transformation|GetActorLocation _partner) "0, 0,20.000000") (Utilities|Array|MakeArray "ObjectTypeQuery3") false 0 "ForOneFrame"))
    (if _returnvalue
      (bind _asbp_guard (Utilities|Casting|CastToBP_Guard (.HitActor (Collision|BreakHitResult _outhit))))
      (Game|Damage|ApplyPointDamage _asbp_guard 5.0 (Transformation|GetActorLocation) (Collision|MakeHitResult false false 0.0 0.0 "0, 0, 0" "0, 0, 0" "0,0,1" "0,0,1" 0 0)))))

(fn ConstructionScript)

(fn CheckforPair
  (bind _filteredtripwires (LocalVariables|GetFilteredTripWires))
  (bind _outactors (Actor|GetAllActorsOfClass "BP_TripWire_C"))
  (for _array_element _outactors
    (if (!= _array_element self)
      ;[1 1 1] Pair check
      (if (not (Utilities|IsValid (Variables|BP_TripWire_C|Getpartner _array_element)))
        ;[1 1 1] check if within range
        (if (<= (Math|Vector|Distance(Vector) (Transformation|GetActorLocation _array_element) (Transformation|GetActorLocation)) (Variables|Default|GetMaxRange))
          ;[1 1 1] check for line of sight
          (bind _outhit (Collision|LineTraceForObjects (+ (Transformation|GetActorLocation _array_element) (Variables|/Script/Engine.SceneComponent|GetRelativeLocation (Variables|Default|GetStaticMesh))) (+ (Transformation|GetActorLocation) (Variables|/Script/Engine.SceneComponent|GetRelativeLocation (Variables|Default|GetStaticMesh))) (Utilities|Array|MakeArray "ObjectTypeQuery2" "ObjectTypeQuery1") false 0 "Persistent"))
          (if (== (.HitActor (Collision|BreakHitResult _outhit)) _array_element)
            (Utilities|Map|Add (LocalVariables|GetFilteredTripWires) _array_element (Transformation|GetDistanceTo _array_element self)))))))
  (bind _keys (Utilities|Map|Keys _filteredtripwires))
  (bind _output_get (LocalVariables|SetClosestObjects (Utilities|Array|Get(acopy) _keys)))
  (LocalVariables|SetMinimumDistance (.Value (Utilities|Map|Find _filteredtripwires _output_get)))
  (bind _values (Utilities|Map|Values (LocalVariables|GetFilteredTripWires)))
  (for (_array_element_2 _array_index) _values
    (if (< _array_element_2 (LocalVariables|GetMinimumDistance))
      (LocalVariables|SetMinimumDistance _array_element_2)
      (bind _keys_2 (Utilities|Map|Keys (LocalVariables|GetFilteredTripWires)))
      (LocalVariables|SetClosestObjects (Utilities|Array|Get(acopy) _keys_2 _array_index))))
  (return (LocalVariables|GetClosestObjects)))