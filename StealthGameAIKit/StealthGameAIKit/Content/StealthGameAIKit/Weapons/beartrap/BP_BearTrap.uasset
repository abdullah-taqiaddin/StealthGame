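; Bear trap actor that snaps shut on a character who steps into it and deals point damage.
; A character leaving the trigger box sets the Activated flag, and later overlaps only spring the trap while it is set.
; A DoOnce with no reset makes it single-use, playing the close montage on the skeletal mesh and applying damage as the montage starts.
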(event OnComponentBeginOverlap(Box)
  (params (OverlappedComponent :type Primitive%20Component%20Object%20Reference) (OtherActor :type Actor%20Object%20Reference) (OtherComp :type Primitive%20Component%20Object%20Reference) (OtherBodyIndex :type Integer) (bFromSweep :type Boolean) (SweepResult :type Hit%20Result%20Structure%20%28by%20ref%29))
  (if (Variables|Default|GetActivated)
    (bind _ascharacter (Utilities|Casting|CastToCharacter OtherActor))
    (Utilities|FlowControl|DoOnce false
      (:Completed
        (Animation|Montage|PlayMontage (Variables|Default|GetSkeletalMesh) "/Game/Animations/BearTrap/Mesh/BearTrap_AnimClose_Montage.BearTrap_AnimClose_Montage"
          (:then
            (Game|Damage|ApplyPointDamage _ascharacter 1e+02 (Transformation|GetActorLocation) (Collision|MakeHitResult false false 0.0 0.0 "0, 0, 0" "0, 0, 0" "0,0,1" "0,0,1" 0 0) 0 self)))))))

(event OnComponentEndOverlap(Box)
  (params (OverlappedComponent :type Primitive%20Component%20Object%20Reference) (OtherActor :type Actor%20Object%20Reference) (OtherComp :type Primitive%20Component%20Object%20Reference) (OtherBodyIndex :type Integer))
  (Utilities|Casting|CastToCharacter OtherActor)
  (Variables|Default|SetActivated true))

(event Collision|EventActorBeginOverlap
  (params (OtherActor :type Actor%20Object%20Reference)))

(event EventTick
  (params (DeltaSeconds :type Float%20%28single-precision%29)))

(fn ConstructionScript)