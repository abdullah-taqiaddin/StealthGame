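; BP_Goal is the escape goal: an overlap trigger that plays a getaway cinematic when the player reaches it.
; Tick feeds Sphere3's location to the marker widget to update its distance text.
; If CanEscape is set and Played is not, overlap calls DisableInput, hides the player HUD and plays GetawaySequencer.
; After a fixed delay, it advances the objective, restores the HUD, hides the marker and destroys Sphere3, provided the objective widget is valid.
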(event OnComponentBeginOverlap(Sphere)
  (params (OverlappedComponent :type Primitive%20Component%20Object%20Reference) (OtherActor :type Actor%20Object%20Reference) (OtherComp :type Primitive%20Component%20Object%20Reference) (OtherBodyIndex :type Integer) (bFromSweep :type Boolean) (SweepResult :type Hit%20Result%20Structure%20%28by%20ref%29))
  ;[1 1 1] PlaySequence
  (if (== (Utilities|GetClass OtherActor) "/Game/StealthGameAIKit/Characters/Player/BP_Player.BP_Player_C")
    (if (not (Variables|Default|Getplayed))
      (if (Variables|Default|GetCanEscape)
        (bind _asbp_player (Utilities|Casting|CastToBP_Player (Game|Player|GetPlayerPawn 0)))
        (Input|DisableInput 0)
        (Widget|SetVisibility (Variables|/Game/StealthGameAIKit/Characters/Player/BP_Player.BP_Player_C|GetMainWidget _asbp_player) "Hidden")
        (bind _returnvalue (Sequencer|Player|CreateLevelSequencePlayer "/Game/Cinematics/GetawaySequencer.GetawaySequencer"))
        (Sequencer|Player|Play _returnvalue :!class /Script/MovieScene.MovieSceneSequencePlayer)
        (Utilities|FlowControl|Delay 8.9)
        (bind _asbp_base_character (Utilities|Casting|CastToBP_BaseCharacter (Game|Player|GetPlayerPawn 0)))
        (Utilities|IsValid (Variables|/Game/StealthGameAIKit/Characters/Base/BP_BaseCharacter.BP_BaseCharacter_C|GetObjectiveWidget _asbp_base_character)
          (:Is%20Valid
            (Default|UpdateObjective (Variables|/Game/StealthGameAIKit/Characters/Base/BP_BaseCharacter.BP_BaseCharacter_C|GetObjectiveWidget _asbp_base_character) 3)
            (bind _asbp_player_2 (Utilities|Casting|CastToBP_Player (Game|Player|GetPlayerPawn 0)))
            (Widget|SetVisibility (Variables|/Game/StealthGameAIKit/Characters/Player/BP_Player.BP_Player_C|GetMainWidget _asbp_player_2) "Visible")
            (Development|SetHiddeninGame (Variables|Default|GetMarkerWidget) true false)
            (Variables|Default|Setplayed true)
            (Rendering|SetVisibility (Variables|Default|GetSphere) true false)
            (Components|DestroyComponent (Variables|Default|GetSphere_3))))))))

(event EventTick
  (params (DeltaSeconds :type Float%20%28single-precision%29))
  ;[1 1 1] TrackDistance
  (bind _aswbp_marker (Utilities|Casting|CastToWBP_Marker (UserInterface|GetWidget (Variables|Default|GetMarkerWidget))))
  (Default|UpdateDistanceText _aswbp_marker (Transformation|GetWorldLocation (Variables|Default|GetSphere_3))))

(fn ConstructionScript)