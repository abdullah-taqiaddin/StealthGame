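; Base weapon actor for BP_BaseCharacter owners, handling equipping, hitscan firing, ammo and reloading.
; While the owner aims, Fire line-traces within a random cone, spawns trail, sound and impact effects, and applies point damage, zeroed for the filter class.
; Owner dispatchers drive reload state and mesh visibility on weapon switch.
; Shots and reloads update clip and reserve ammo, notifying widgets through dispatchers and signalling when a reload is needed.
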(event Custom|BindingOwnerEventDispatchers
  ;[1 1 1] Bind Owner Event Dispatchers
  (EventDispatchers|AssignOnBeginReload (Variables|Reference|GetOwnerPawn) (EventDispatchers|CreateEvent :!event Custom|BeginReload))
  (EventDispatchers|BindEventtoOnEndReloaded (Variables|Reference|GetOwnerPawn) (EventDispatchers|CreateEvent :!event Custom|EndReload))
  (EventDispatchers|AssignOnBeginAim (Variables|Reference|GetOwnerPawn) (EventDispatchers|CreateEvent :!event Custom|BeginAim))
  (EventDispatchers|AssignOnEndAim (Variables|Reference|GetOwnerPawn) (EventDispatchers|CreateEvent :!event Custom|EndAim))
  (EventDispatchers|BindEventtoOnSwitchWeaponFinished (Variables|Reference|GetOwnerPawn) (EventDispatchers|CreateEvent :!event Custom|ShowWeaponMeshes)))

(event Custom|ShowWeaponMeshes
  (params (NewWeapon :type BP%20Base%20Weapon%20Object%20Reference))
  ;[1 1 1] Show Weapon Meshes
  (if (== NewWeapon self)
    (Rendering|SetVisibility (Variables|Default|GetWeaponSkeletalMesh) true false)))

(event Custom|BeginReload
  ;[1 1 1] Event Dispatch [Begin Reload]
  (if (Getter|IsOwnerEquipThisWeapon)
    (Variables|Status|SetbIsReloading true)))

(event Custom|BeginAim
  ;[1 1 1] Override Events
)

(event Custom|EndAim
  ;[1 1 1] Override Events
)

(event Custom|UnEquipped
  ;[1 1 1] Un Equipped
  (Rendering|SetVisibility (Variables|Default|GetWeaponSkeletalMesh) false false))

(event Custom|Equipped
  ;[1 1 1] Weapon Equipped
  (Transformation|AttachComponentToComponent (Variables|/Script/Engine.Character|GetMesh (Variables|Reference|GetOwnerPawn)) "Weapon" "SnapToTarget" "SnapToTarget" "KeepRelative" true)
  (CallFunction|BindingOwnerEventDispatchers)
  (Default|CallOnUpdateWidget (Variables|Config|Status|GetWeaponData)))

(event Custom|Fire
  (params (Direction :type Vector) (RandomHalfAngle :type Float%20%28single-precision%29) (FilterClass :type BP%20Base%20Character%20Class%20Reference))
  ;[1 1 1] Fire
  (if (Variables|/Game/StealthGameAIKit/Characters/Base/BP_BaseCharacter.BP_BaseCharacter_C|GetbAiming (Variables|Reference|GetOwnerPawn))
    (Utilities|FlowControl|Sequence
      (:then_0
        (Variables|LineTrace|SetShootDirection Direction)
        (Variables|LineTrace|SetRandomConeHalfAngle RandomHalfAngle)
        (Variables|LineTrace|SetTraceFilterClass FilterClass))
      (:then_1
        (if (or (Variables|Config|Status|GetbInfiniteAmmo) (and (not (Variables|Status|GetbIsReloading)) (not (Getter|IsEmptyAmmo))))
          (Transformation|SetWorldRotation (Variables|Default|GetMuzzle) (Math|Rotator|MakeRotfromX (Variables|LineTrace|GetShootDirection)) false false)
          (Utilities|FlowControl|Sequence
            (:then_0
              ;;[1 1 1] Calculate Trace Start & Trace End Locations
              (Variables|LineTrace|SetTraceStart (Transformation|GetWorldLocation (Variables|Default|GetMuzzle)))
              (Variables|LineTrace|SetTraceEnd (+ (Variables|LineTrace|GetTraceStart) (Trace|GetRandomScalingDirection (Variables|LineTrace|GetShootDirection) (Variables|LineTrace|GetRandomConeHalfAngle) (Variables|Status|GetFireRange))))
              (bind _outhit (Collision|LineTraceByChannel (Variables|LineTrace|GetTraceStart) (Variables|LineTrace|GetTraceEnd) "TraceTypeQuery5" false (Utilities|Array|MakeArray (Variables|Reference|GetOwnerPawn)) "None" true "(R=0.000000,G=0.219207,B=1.000000,A=1.000000)"))
              (Utilities|FlowControl|Sequence
                (:then_0
                  (Variables|LineTrace|SetTraceHitResult _outhit))
                (:then_1
                  (Variables|LineTrace|SetTraceHit (.bBlockingHit (Collision|BreakHitResult _outhit))))
                (:then_2
                  (Variables|LineTrace|SetTraceHitLocation (.Location (Collision|BreakHitResult _outhit))))
                (:then_3
                  (Variables|LineTrace|SetTraceHitActor (.HitActor (Collision|BreakHitResult _outhit))))))
            (:then_1
              (Effects|SpawnFireEffects)
              (Default|CallOnFire)
              (if (Variables|LineTrace|GetTraceHit)
                ;;[1 1 1] Apply Damage
                (Game|Damage|ApplyPointDamage (Variables|LineTrace|GetTraceHitActor) (Math|Conversions|ToFloat(Boolean) (!= (Utilities|GetClass (Variables|LineTrace|GetTraceHitActor)) (Variables|LineTrace|GetTraceFilterClass))) (Trace|GetTraceDirection) (Variables|LineTrace|GetTraceHitResult) (Pawn|GetController (Variables|Reference|GetOwnerPawn)) self)
                ;;[1 1 1] Bullet Impact Effect
                (Effects|SpawnEmitteratLocation (Variables|Config|Effect|GetBulletImpact) (Variables|LineTrace|GetTraceHitLocation) "0, 0, 0" "0.200000,0.200000,0.200000" true "AutoRelease")))
            (:then_2
              ;;[1 1 1] Decrease Ammo & Check I Need Reload
              (Math|Integer|DecrementInt (.currentammoinclip (Variables|Config|Status|GetWeaponData))
                (:%20%20
                  (Default|CallOnUpdateWidget (Variables|Config|Status|GetWeaponData))
                  (if (and (<= (.currentammoinclip (Variables|Config|Status|GetWeaponData)) 0) (not (Getter|IsEmptyAmmo)))
                    (Default|CallOnNeedReload)))))))))))

(event Custom|EndReload
  (bind (_newcurrentammo _newammoinclip) (Ammo|CalcAmmoAfterReload))
  (bind _weapondata (Variables|Config|Status|GetWeaponData))
  ;[1 1 1] Event Dispatch [End Reload]
  (if (not (Variables|Config|Status|GetbInfiniteAmmo))
    (if (Getter|IsOwnerEquipThisWeapon)
      (Utilities|Struct|SetmembersinFWeaponData (Variables|Config|Status|GetWeaponData) _newcurrentammo _newammoinclip)
      (Default|CallOnUpdateWidget (Variables|Config|Status|GetWeaponData) :!label _label)
      (Variables|Status|SetbIsReloading false))
    (else
      (Utilities|Struct|SetmembersinFWeaponData _weapondata (Utilities|Struct|BreakFWeaponData _weapondata))
      (goto _label))))

(event EventBeginPlay
  ;[1 1 1] Comment
  (Rendering|SetVisibility (Variables|Default|GetWeaponSkeletalMesh) false false)
  (Variables|Reference|SetOwnerPawn (.AsBP%20Base%20Character (Utilities|Casting|CastToBP_BaseCharacter (Components|GetOwner)))))

(fn ConstructionScript)

(fn IsEmptyAmmo
  (LocalVariables|SetEmptyAmmo (<= (.currentammo (Variables|Config|Status|GetWeaponData)) 0))
  (LocalVariables|SetEmptyClip (<= (.currentammoinclip (Variables|Config|Status|GetWeaponData)) 0))
  (return (and (LocalVariables|GetEmptyAmmo) (LocalVariables|GetEmptyClip))))

(fn GetMuzzleLocation
  (return (Transformation|GetWorldLocation (Variables|Default|GetMuzzle))))

(fn IsOwnerEquipThisWeapon
  (Utilities|IsValid (Variables|Reference|GetOwnerPawn)
    (:Is%20Valid
      (LocalVariables|SetOwnerWeaponClass (Utilities|GetClass (Variables|/Game/StealthGameAIKit/Characters/Base/BP_BaseCharacter.BP_BaseCharacter_C|GetCurrentWeapon (Variables|Reference|GetOwnerPawn))))
      (return (== (LocalVariables|GetOwnerWeaponClass) (Utilities|GetClass self))))
    (:Is%20Not%20Valid
      (return false))))

(fn GiveAmmo
  (params (Amount :type Integer))
  (Utilities|Struct|SetmembersinFWeaponData (Variables|Config|Status|GetWeaponData) (+ Amount (.currentammo (Variables|Config|Status|GetWeaponData))))
  (if (Getter|IsOwnerEquipThisWeapon)
    (Default|CallOnUpdateWidget (Variables|Config|Status|GetWeaponData))
    (return)
    (else
      (return))))

(fn GetTraceDirection
  (return (Math|Vector|Normalize (- (Variables|LineTrace|GetTraceEnd) (Variables|LineTrace|GetTraceStart)))))

(fn GetRandomScalingDirection
  (params (Direction :type Vector) (ConeHalfInDegree :type Float%20%28single-precision%29) (ScaleLength :type Float%20%28single-precision%29))
  (return (* (Math|Random|RandomUnitVectorinConeinDegrees Direction ConeHalfInDegree) ScaleLength)))

(fn CalcAmmoAfterReload
  (bind _weapondata (Variables|Config|Status|GetWeaponData))
  (bind _weapondata_2 (Variables|Config|Status|GetWeaponData))
  (bind (_currentammo _currentammoinclip _ammoperclip) (Utilities|Struct|BreakFWeaponData _weapondata_2))
  (bind (_currentammo_2 _currentammoinclip_2) (Utilities|Struct|BreakFWeaponData _weapondata))
  (LocalVariables|SetUseAmmo (- _ammoperclip _currentammoinclip))
  (return (|(CurrentAmmo-(min(CurrentAmmo,{05494A5D-4B81-309C-AC5A-799CED488916}))) (.CurrentAmmo (Utilities|Struct|BreakFWeaponData (Variables|Config|Status|GetWeaponData)))) (|(CurrentAmmoInClip+(min(CurrentAmmo,{05494A5D-4B81-309C-AC5A-799CED488916}))) _currentammo_2 _currentammoinclip_2)))

(fn SpawnFireEffects
  ;[1 1 1] Bullet Trace Effect
  (bind _returnvalue (Effects|SpawnEmitteratLocation "/Game/StealthGameAIKit/Weapons/Handgun/P_BulletTrail.P_BulletTrail" (Variables|LineTrace|GetTraceStart)))
  (Effects|Components|ParticleSystem|SetVectorParameter _returnvalue "BeamTarget" (Math|Vector|SelectVector (Variables|LineTrace|GetTraceHitLocation) (Variables|LineTrace|GetTraceEnd) (Variables|LineTrace|GetTraceHit)))
  ;[1 1 1] Play Gunfire Sound
  (Audio|PlaySoundatLocation (Variables|Config|Audio|GetFireSound) (Transformation|GetWorldLocation (Variables|Default|GetMuzzle)) "0, 0, 0" 0.5 1.0 0.0 "/Game/StealthGameAIKit/Weapons/Handgun/ATT_FirstPersonTemplateWeaponFire02.ATT_FirstPersonTemplateWeaponFire02" 0 0)
  (return))

(fn GetMuzzleDirection
  (return (Math|Vector|GetForwardVector (Transformation|GetWorldRotation (Variables|Default|GetMuzzle)))))