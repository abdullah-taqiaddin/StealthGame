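; BP_NoiseGadget is a launched projectile that makes an AI-audible noise where it hits.
; BeginPlay sets the projectile movement velocity from LaunchVelocity.
; Hits on anything but the player report noise at a fixed range as the player, then destroy the actor after a delay.
; Mesh overlap only prints debug text, and an unconnected branch holds a variable-range, navmesh-projected pulse effect version that never runs.
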(event OnComponentBeginOverlap(GadgetCollision)
  (params (OverlappedComponent :type Primitive%20Component%20Object%20Reference) (OtherActor :type Actor%20Object%20Reference) (OtherComp :type Primitive%20Component%20Object%20Reference) (OtherBodyIndex :type Integer) (bFromSweep :type Boolean) (SweepResult :type Hit%20Result%20Structure%20%28by%20ref%29))
  ;[1 1 1] Report Noise
)

(event OnComponentBeginOverlap(GadgetMesh)
  (params (OverlappedComponent :type Primitive%20Component%20Object%20Reference) (OtherActor :type Actor%20Object%20Reference) (OtherComp :type Primitive%20Component%20Object%20Reference) (OtherBodyIndex :type Integer) (bFromSweep :type Boolean) (SweepResult :type Hit%20Result%20Structure%20%28by%20ref%29))
  (Development|PrintString (Utilities|GetDisplayName OtherComp)))

(event EventBeginPlay
  ;[1 1 1] Initialize
  (Variables|/Script/Engine.MovementComponent|SetVelocity (Variables|Default|GetProjectileMovement1) (Variables|Config|GetLaunchVelocity)))

(event Collision|EventHit
  (params (MyComp :type Primitive%20Component%20Object%20Reference) (Other :type Actor%20Object%20Reference) (OtherComp :type Primitive%20Component%20Object%20Reference) (bSelfMoved :type Boolean) (HitLocation :type Vector :default "0, 0, 0") (HitNormal :type Vector :default "0, 0, 0") (NormalImpulse :type Vector :default "0, 0, 0") (Hit :type Hit%20Result%20Structure%20%28by%20ref%29))
  (bind _returnvalue (Game|Player|GetPlayerPawn 0))
  (if (!= Other _returnvalue)
    (Class|AISenseHearing|ReportNoiseEvent HitLocation 1.0 _returnvalue 1e+03 "None")
    (Utilities|FlowControl|Delay 5.0)
    (Actor|DestroyActor)))

(fn ConstructionScript)