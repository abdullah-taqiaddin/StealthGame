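; Launcher weapon that fires noise gadgets, attaching to the player's gadget launcher pivot when equipped.
; While equipped, aiming starts and stops a child-actor throw arc preview, which receives the launcher's noise range at construction.
; Firing requires aiming and ammo, then spawns a noise gadget with velocity along the muzzle arrow and the same noise range, decrements ammo and updates the widget.
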(event EventBeginAim
  ;[1 1 1] Begin Aim & End Aim
  (if (CallFunction|IsOwnerEquipThisWeapon)
    (Default|BeginDrawArc (Variables|Reference|GetArcLineRef) self)))

(event EventEquipped
  ;[1 1 1] Equipped
  (|CallParentFunction)
  (bind _asbp_player (Utilities|Casting|CastToBP_Player (Variables|Default|GetOwnerPawn)))
  (Transformation|AttachComponentToComponent (Variables|/Game/StealthGameAIKit/Characters/Player/BP_Player.BP_Player_C|GetGadgetLauncherPivot _asbp_player) "None" "SnapToTarget" "SnapToTarget" "KeepRelative" true))

(event EventFire
  (params (Direction :type Vector :default "0, 0, 0") (RandomHalfAngle :type Float%20%28single-precision%29) (FilterClass :type BP%20Base%20Character%20Class%20Reference))
  ;[1 1 1] Fire
  (if (Variables|/Game/StealthGameAIKit/Characters/Base/BP_BaseCharacter.BP_BaseCharacter_C|GetbAiming (Variables|Default|GetOwnerPawn))
    (if (not (CallFunction|IsEmptyAmmo))
      (Game|SpawnActorfromClass "/Game/StealthGameAIKit/Weapons/NoiseGadget/BP_NoiseGadget.BP_NoiseGadget_C" (Transformation|GetActorTransform) "Undefined" self (* (Math|Vector|GetForwardVector (Variables|Default|GetMuzzleDirectionArrow)) (Variables|Status|GetLaunchVelocityPower)) (Variables|Config|GetNoiseRange) (Variables|Default|GetOwnerPawn))
      (Math|Integer|DecrementInt (.currentammo (Variables|Default|GetWeaponData))
        (:%20%20
          (Default|CallOnUpdateWidget (Variables|Default|GetWeaponData)))))))

(event EventEndAim
  ;[1 1 1] Begin Aim & End Aim
  (if (CallFunction|IsOwnerEquipThisWeapon)
    (Default|EndDrawArc (Variables|Reference|GetArcLineRef))))

(event EventBeginPlay
  ;[1 1 1] Begin Play
  (|CallParentFunction)
  (Variables|Reference|SetArcLineRef (.AsBP%20Throw%20Arc%20Line (Utilities|Casting|CastToBP_ThrowArcLine (Variables|/Script/Engine.ChildActorComponent|GetChildActor (Variables|Default|GetArcLine))))))

(fn ConstructionScript
  (Variables|/Game/StealthGameAIKit/Weapons/NoiseGadget/BP_ThrowArcLine.BP_ThrowArcLine_C|SetNoiseRange (.AsBP%20Throw%20Arc%20Line (Utilities|Casting|CastToBP_ThrowArcLine (Variables|/Script/Engine.ChildActorComponent|GetChildActor (Variables|Default|GetArcLine)))) (Variables|Config|GetNoiseRange)))