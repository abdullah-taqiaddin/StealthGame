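; Stealth game mode that tracks key collection and shows the game-over and game-clear screens.
; BeginPlay pauses and hides the helicopter, binds the player's death event and counts all BP_Key actors as the collectible target.
; Pickups decrement that count and fire OnCompleteCollectible at zero, which the Debug event forces.
; Player death and EnterGoal open the same widget with different GameClear flags; virtual-joystick platform logic is left disconnected.
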(event Custom|PickupCollectible
  (bind _result (Math|Integer|DecrementInt (Variables|Default|GetTargetCollectibleCount))
    (:%20%20
      (if (<= _result 0)
        (Default|CallOnCompleteCollectible)))))

(event Custom|EnterGoal
  ;[1 1 1] Game Clear
  (bind _returnvalue (UserInterface|CreateWidget "/Game/StealthGameAIKit/UserInterface/WBP_GameOverAndClearScreen.WBP_GameOverAndClearScreen_C" (Game|GetPlayerController 0) true))
  (UserInterface|Viewport|AddtoViewport _returnvalue 0))

(event Custom|PlayerDead
  (bind _returnvalue (UserInterface|CreateWidget "/Game/StealthGameAIKit/UserInterface/WBP_GameOverAndClearScreen.WBP_GameOverAndClearScreen_C" (Game|GetPlayerController 0)))
  (UserInterface|Viewport|AddtoViewport _returnvalue 0))

(event Custom|Debug
  (Variables|Default|SetTargetCollectibleCount 0)
  (if (<= (stale Custom|PickupCollectible _result) 0)
    (Default|CallOnCompleteCollectible)))

(event EventBeginPlay
  ;[1 1 1] Set Heli hidden in game
  (bind _returnvalue (Actor|GetActorOfClass "/Game/Helicopter_Dekohawk/Blueprints/BP_Deko_Hawk_01a.BP_Deko_Hawk_01a_C"))
  (Class|AudioComponent|SetPaused (Variables|/Game/Helicopter_Dekohawk/Blueprints/BP_Deko_Hawk_01a.BP_Deko_Hawk_01a_C|GetEngine _returnvalue) true)
  (Rendering|SetActorHiddenInGame _returnvalue true)
  (EventDispatchers|BindEventtoOnPlayerDead (.AsBP%20Player (Utilities|Casting|CastToBP_Player (Game|GetPlayerCharacter 0))) (delegate Custom|PlayerDead))
  (bind _outactors (Actor|GetAllActorsOfClass "/Game/StealthGameAIKit/Placeables/Pickups/Collectible/BP_Key.BP_Key_C"))
  (Variables|Default|SetTargetCollectibleCount (Utilities|Array|Length _outactors))
  (EventDispatchers|AssignOnPickupCollectible _outactors (delegate Custom|PickupCollectible)))

(fn ConstructionScript)