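; Placeable patrol route spline that supplies AI with waypoint destinations, as either a closed loop or a back-and-forth path.
; The construction script applies the loop setting, labels each spline point with its index and spaces arrow meshes evenly along the length.
; GetNextDestination takes the caller's index and direction, returning the next world location, index and direction, wrapping on loops or flipping direction after stepping past an end.
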(event EventBeginPlay)

(event Collision|EventActorBeginOverlap
  (params (OtherActor :type Actor%20Object%20Reference)))

(event EventTick
  (params (DeltaSeconds :type Float%20%28single-precision%29)))

(fn ConstructionScript
  (Variables|Config|SetNum%20Meshes (Math|Integer|Max(Integer) (Variables|Config|GetNum%20Meshes) (Spline|GetNumberOfSplinePoints (Variables|Default|GetSpline))))
  (Spline|SetClosedLoop (Variables|Default|GetSpline) (Variables|Config|GetbIsLoop) true)
  (for _index (range 0 (- (Variables|Config|GetNum%20Meshes) 1))
    (if (< _index (Spline|GetNumberOfSplinePoints (Variables|Default|GetSpline)))
      (CallFunction|ShowSplinePointIndex _index))
    (CallFunction|AddArrowMeshComponent (- (Variables|Config|GetNum%20Meshes) 1) _index)))

(fn GetNextDestination
  (params (Current%20Waypoint%20Index :type Integer) (PatrolDirectionForward :type Boolean))
  (LocalVariables|SetDirectionForward PatrolDirectionForward)
  (Utilities|FlowControl|Sequence
    (:then_0
      (if (Variables|Config|GetbIsLoop)
        (LocalVariables|SetNextIndex (|((CurrentWaypointIndex+1)%SplinePoints) Current%20Waypoint%20Index (Spline|GetNumberOfSplinePoints (Variables|Default|GetSpline))))
        (elif PatrolDirectionForward
          (bind _output_get (LocalVariables|SetNextIndex (+ Current%20Waypoint%20Index 1)))
          (if (> _output_get (- (Spline|GetNumberOfSplinePoints (Variables|Default|GetSpline)) 1))
            (LocalVariables|SetDirectionForward false))
          (else
            (bind _output_get_2 (LocalVariables|SetNextIndex (- Current%20Waypoint%20Index 1)))
            (if (< _output_get_2 0)
              (LocalVariables|SetDirectionForward true))))))
    (:then_1
      (return (Spline|GetLocationatSplinePoint (Variables|Default|GetSpline) (LocalVariables|GetNextIndex) "World") (LocalVariables|GetNextIndex) (LocalVariables|GetDirectionForward)))))

(fn ShowSplinePointIndex
  (params (SplinePointIndex :type Integer))
  (LocalVariables|SetRenderText (Utilities|Text|ToText(Integer) SplinePointIndex))
  (LocalVariables|SetSplinePoint (Spline|GetLocationatSplinePoint (Variables|Default|GetSpline) SplinePointIndex "Local"))
  (bind _returnvalue (AddComponent|AddTextRenderComponent false (Math|Transform|MakeTransform (+ (LocalVariables|GetSplinePoint) "0, 0,50.000000") "45.000000,180.000000, 0" "1,1,1")))
  (Rendering|Components|TextRender|SetText _returnvalue (LocalVariables|GetRenderText))
  (return))

(fn AddArrowMeshComponent
  (params (NumberOfMeshes :type Integer) (Index :type Integer))
  (bind _spline (Variables|Default|GetSpline))
  (LocalVariables|SetDistance (|(MeshIndex*(SplineLength/NumberOfMeshes)) Index (Spline|GetSplineLength (Variables|Default|GetSpline)) NumberOfMeshes))
  (AddComponent|AddStaticMeshComponent false (Math|Transform|MakeTransform (Math|Transform|InverseTransformLocation (Transformation|GetActorTransform) (Spline|GetLocationatDistanceAlongSpline _spline (LocalVariables|GetDistance) "World")) (Spline|GetRotationatDistanceAlongSpline _spline (LocalVariables|GetDistance) "Local") "3.000000,3.000000,3.000000"))
  (return))