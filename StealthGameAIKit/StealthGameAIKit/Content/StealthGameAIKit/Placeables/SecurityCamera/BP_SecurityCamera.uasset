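; Possessable security camera pawn that sweeps on a timeline until the player views through it to look, zoom and mark guards.
; Becoming view target stops the sweep, applies rotation-relative view limits and starts a looping timer, likely driving the guard-marking line trace.
; A sphere trace hops between cameras using a blended view-target switch before possession.
; Leaving, or the FoundPlayerCharacter event, restores view limits and returns control to BP_Player.
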(event Custom|GuardSpotted
  (bind _returnvalue (Utilities|SpottableDistance))
  (bind (_from _to) (CallFunction|CalcTraceLinefromPlayerCamera _returnvalue))
  ;[1 1 1] Spotted
  (bind _outhit (Class|KismetSystemLibrary|LineTraceSinglebyProfile _from _to "GuardPawn" false 0 "None" true))
  (bind _asbp_guard (Utilities|Casting|CastToBP_Guard (.hitactor _outhit)))
  (Default|MarkIndicator _asbp_guard))

(event Custom|StopSwingTimeline
  ;[1 1 1] Begin Play
  (bind _alpha (Timeline|SwingCamera Stop)
    (:Update
      (Transformation|SetRelativeRotation (Variables|Default|GetRotatePivot) (Math|Rotator|MakeRotator 0.0 0.0 (* _alpha (Variables|Status|GetSwingAngle))) false false))))

(event Custom|PlaySwingTimeline
  ;[1 1 1] Begin Play
  (bind _alpha (Timeline|SwingCamera Play)
    (:Update
      (Transformation|SetRelativeRotation (Variables|Default|GetRotatePivot) (Math|Rotator|MakeRotator 0.0 0.0 (* _alpha (Variables|Status|GetSwingAngle))) false false))))

(event Custom|TransitionCameraView
  (params (TargetPawn :type Pawn%20Object%20Reference))
  ;[1 1 1] Transition Camera View
  (Game|Player|SetViewTargetwithBlend (Game|GetPlayerController 0) TargetPawn 0.5 "VTBlend_Cubic" 3.0 false)
  (Utilities|FlowControl|Delay 0.5)
  (Utilities|FlowControl|Sequence
    (:then_0
      (Pawn|UnPossess (Game|GetPlayerController 0))
      (Pawn|Possess (Game|GetPlayerController 0) TargetPawn)
      (Variables|/Script/Engine.CameraComponent|SetFieldOfView (Variables|Default|GetCamera) (Utilities|DefaultCameraFOV)))
    (:then_1
      (CallFunction|PlaySwingTimeline)
      (Utilities|Time|ClearandInvalidateTimerbyHandle (Variables|EventTimer|GetTimerGuardSpotted))
      (Components|Tick|SetComponentTickEnabled (Variables|Default|GetSpringArm) false))))

(event Custom|FoundPlayerCharacter
  ;[1 1 1] Leave Camera
  (Utilities|FlowControl|Sequence
    (:then_0
      (Camera|SetCameraAngle (Variables|Status|GetDefaultCameraView))
      (Utilities|Time|ClearandInvalidateTimerbyHandle (Variables|EventTimer|GetTimerGuardSpotted)))
    (:then_1
      (bind _outactors (Actor|GetAllActorsOfClass "/Game/StealthGameAIKit/Characters/Player/BP_Player.BP_Player_C"))
      (Variables|Reference|SetPlayerRef (Utilities|Array|Get(acopy) _outactors))
      (CallFunction|TransitionCameraView (Variables|Reference|GetPlayerRef)))))

(event EventBeginPlay
  (bind _returnvalue (Game|GetPlayerCameraManager 0))
  ;[1 1 1] Begin Play
  (Variables|Status|SetDefaultCameraView (Utilities|Struct|MakeFCameraViewParameter (Variables|/Script/Engine.PlayerCameraManager|GetViewPitchMin _returnvalue) (Variables|/Script/Engine.PlayerCameraManager|GetViewPitchMax _returnvalue) (Variables|/Script/Engine.PlayerCameraManager|GetViewYawMin _returnvalue) (Variables|/Script/Engine.PlayerCameraManager|GetViewYawMax _returnvalue)))
  (Components|Tick|SetComponentTickEnabled (Variables|Default|GetSpringArm) false)
  (bind _alpha (Timeline|SwingCamera Play)
    (:Update
      (Transformation|SetRelativeRotation (Variables|Default|GetRotatePivot) (Math|Rotator|MakeRotator 0.0 0.0 (* _alpha (Variables|Status|GetSwingAngle))) false false))))

(event EventOnBecomeViewTarget
  (params (PC :type Player%20Controller%20Object%20Reference))
  (bind (_newpitchmin _newpitchmax _newyawmin _newyawmax) (Camera|MakeNewCameraAngle))
  ;[1 1 1] Possessed
  (Camera|SetCameraAngle (Utilities|Struct|MakeFCameraViewParameter _newpitchmin _newpitchmax _newyawmin _newyawmax))
  (bind _returnvalue (Utilities|Time|SetTimerbyEvent (EventDispatchers|CreateEvent :!event Custom|GuardSpotted) 0.5 true))
  (Variables|EventTimer|SetTimerGuardSpotted _returnvalue)
  (CallFunction|StopSwingTimeline)
  (Components|Tick|SetComponentTickEnabled (Variables|Default|GetSpringArm) true))

(event Input|ActionEvents|InputActionHackingToCamera
  (params (Key :type Key%20Structure :default "None"))
  (bind _returnvalue (Utilities|HackableDistance))
  (bind (_from _to) (CallFunction|CalcTraceLinefromPlayerCamera _returnvalue))
  ;[1 1 1] Hacking to other camera
  (:Pressed
    (bind _outhit (Collision|SphereTraceByChannel _from _to 1e+01 "TraceTypeQuery6" false 0 "None"))
    (bind _asbp_security_camera (Utilities|Casting|CastToBP_SecurityCamera (.hitactor _outhit)))
    (bind _output_get (Variables|Reference|SetTargetCamera _asbp_security_camera))
    (CallFunction|TransitionCameraView _output_get)))

(event Input|ActionEvents|InputActionLeaveCamera
  (params (Key :type Key%20Structure :default "None"))
  ;[1 1 1] Leave Camera
  (:Pressed
    (Utilities|FlowControl|Sequence
      (:then_0
        (Camera|SetCameraAngle (Variables|Status|GetDefaultCameraView))
        (Utilities|Time|ClearandInvalidateTimerbyHandle (Variables|EventTimer|GetTimerGuardSpotted)))
      (:then_1
        (bind _outactors (Actor|GetAllActorsOfClass "/Game/StealthGameAIKit/Characters/Player/BP_Player.BP_Player_C"))
        (Variables|Reference|SetPlayerRef (Utilities|Array|Get(acopy) _outactors))
        (CallFunction|TransitionCameraView (Variables|Reference|GetPlayerRef))))))

(event Input|ActionEvents|InputActionZoomIn
  (params (Key :type Key%20Structure :default "None"))
  ;[1 1 1] Zoom in / out
  (:Pressed
    (Variables|/Script/Engine.CameraComponent|SetFieldOfView (Variables|Default|GetCamera) (|(Clamp((FOV-Rate),45,90)) (Variables|/Script/Engine.CameraComponent|GetFieldOfView (Variables|Default|GetCamera)) (Utilities|ZoominOutRate)))))

(event Input|ActionEvents|InputActionZoomOut
  (params (Key :type Key%20Structure :default "None"))
  ;[1 1 1] Zoom in / out
  (:Pressed
    (Variables|/Script/Engine.CameraComponent|SetFieldOfView (Variables|Default|GetCamera) (|(Clamp((FOV+Rate),45,90)) (Variables|/Script/Engine.CameraComponent|GetFieldOfView (Variables|Default|GetCamera)) (Utilities|ZoominOutRate)))))

(event Input|AxisEvents|InputAxisTurn
  (params (AxisValue :type Float%20%28single-precision%29))
  ;[1 1 1] Look up & Look turn
  (Pawn|Input|AddControllerYawInput AxisValue))

(event Input|AxisEvents|InputAxisLookUp
  (params (AxisValue :type Float%20%28single-precision%29))
  ;[1 1 1] Look up & Look turn
  (Pawn|Input|AddControllerPitchInput AxisValue))

(fn ConstructionScript)

(fn SetCameraAngle
  (params (NewCameraView :type F%20Camera%20View%20Parameter%20Structure))
  (bind _returnvalue (Game|GetPlayerCameraManager 0))
  (Utilities|FlowControl|Sequence
    (:then_0
      (Variables|/Script/Engine.PlayerCameraManager|SetViewPitchMin _returnvalue (.pitchmin NewCameraView)))
    (:then_1
      (Variables|/Script/Engine.PlayerCameraManager|SetViewPitchMax _returnvalue (.pitchmax NewCameraView)))
    (:then_2
      (Variables|/Script/Engine.PlayerCameraManager|SetViewYawMin _returnvalue (.yawmin NewCameraView)))
    (:then_3
      (Variables|/Script/Engine.PlayerCameraManager|SetViewYawMax _returnvalue (.yawmax NewCameraView)))
    (:then_4
      (return))))

(fn MakeNewCameraAngle
  (bind _returnvalue (Transformation|GetActorRotation))
  (bind _possessedcameraview (Variables|Status|GetPossessedCameraView))
  (return (+ (.pitchmin _possessedcameraview) (.pitch _returnvalue)) (+ (.pitchmax _possessedcameraview) (.pitch _returnvalue)) (+ (.yawmin _possessedcameraview) (.yaw _returnvalue)) (+ (.yawmax _possessedcameraview) (.yaw _returnvalue))))