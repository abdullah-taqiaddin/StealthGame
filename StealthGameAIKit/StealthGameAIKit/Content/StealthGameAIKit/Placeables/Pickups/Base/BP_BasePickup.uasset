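; Base pickup actor for the stealth game kit, collected when a BP_Player overlaps its collision component.
; The overlap runs the overridable ApplyPickupEffects event, then sets the Collected flag.
; The base ApplyPickupEffects only calls the OnPickuped dispatcher.
; Activate and Deactivate toggle query collision and mesh visibility, and collection itself does not call Deactivate here.
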(event OnComponentBeginOverlap(PickupCollision)
  (params (OverlappedComponent :type Primitive%20Component%20Object%20Reference) (OtherActor :type Actor%20Object%20Reference) (OtherComp :type Primitive%20Component%20Object%20Reference) (OtherBodyIndex :type Integer) (bFromSweep :type Boolean) (SweepResult :type Hit%20Result%20Structure%20%28by%20ref%29))
  (bind _asbp_player (Utilities|Casting|CastToBP_Player OtherActor))
  (CallFunction|ApplyPickupEffects _asbp_player)
  (Variables|Default|SetCollected true))

(event Custom|Activate
  (Collision|SetCollisionEnabled (Variables|Default|GetPickupCollision) "QueryOnly")
  (Development|SetHiddeninGame (Variables|Default|GetStaticMesh) false false))

(event Custom|Deactivate
  (Collision|SetCollisionEnabled (Variables|Default|GetPickupCollision) "NoCollision")
  (Development|SetHiddeninGame (Variables|Default|GetStaticMesh) true false))

(event Custom|ApplyPickupEffects
  (params (PlayerPawn :type BP%20Player%20Object%20Reference))
  ;[1 1 1] Override
  (Default|CallOnPickuped))

(event EventBeginPlay)

(fn ConstructionScript)