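; Health pickup placeable for the stealth AI kit that restores a small fixed amount of the player's health.
; It overrides ApplyPickupEffects and runs the parent pickup logic only when the player's health is not already at maximum.
; It then adds the health without clamping, fires the player's health update event and plays a 2D breathing sound.
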(event EventApplyPickupEffects
  (params (PlayerPawn :type BP%20Player%20Object%20Reference))
  (bind _maxhealth (Variables|/Game/StealthGameAIKit/Characters/Base/BP_BaseCharacter.BP_BaseCharacter_C|GetMaxHealth PlayerPawn))
  (if (not (== (Variables|/Game/StealthGameAIKit/Characters/Base/BP_BaseCharacter.BP_BaseCharacter_C|GetHealth PlayerPawn) _maxhealth))
    (|CallParentFunction PlayerPawn)
    (bind _output_get (Variables|/Game/StealthGameAIKit/Characters/Base/BP_BaseCharacter.BP_BaseCharacter_C|SetHealth PlayerPawn (+ (Variables|/Game/StealthGameAIKit/Characters/Base/BP_BaseCharacter.BP_BaseCharacter_C|GetHealth PlayerPawn) 2.0)))
    (Default|CallOnUpdateHealth PlayerPawn _output_get _maxhealth)
    (Audio|PlaySound2D "/Game/StealthGameAIKit/SFX/PickupSounds/health/Breathing.Breathing" 1.0 1.0 0.0 0 0)))

(fn ConstructionScript
  (|CallParentFunction))