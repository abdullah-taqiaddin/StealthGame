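; BP_Key is a collectible key pickup that advances the player's key objective and guides them with a marker.
; Each tick it spins the mesh, updates the WBP_Marker distance text and scales the marker down with distance.
; On first pickup it plays a sound, hides itself and increments the player's CollectableCount.
; That count indexes all BP_Key actors to reveal the next marker and updates the objective, passing -1 once all are collected.
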(event Custom|ShowWidget
  ;[1 1 1] Show Widget
  (Development|SetHiddeninGame (Variables|Default|GetWidget) false false))

(event Custom|HideWidget
  ;[1 1 1] Hide Widget
  (Rendering|SetVisibility (Variables|Default|GetWidget) true false))

(event EventApplyPickupEffects
  (params (PlayerPawn :type BP%20Player%20Object%20Reference))
  (bind _mainwidget (Variables|/Game/StealthGameAIKit/Characters/Player/BP_Player.BP_Player_C|GetMainWidget PlayerPawn))
  ;[1 1 1] Update the Objective after the key has been collected
  (Utilities|FlowControl|DoOnce false
    (:Completed
      (Audio|PlaySound2D "/Game/StealthGameAIKit/SFX/PickupSounds/Keys/keychain.keychain" 1.0 1.0 0.0 0 0)
      (Variables|Default|Sethasbeencollected true)
      (Default|CallOnPickupCollectible)
      (Rendering|SetActorHiddenInGame true)
      (Development|SetHiddeninGame (Variables|Default|Getdoorkey) true false)
      (Utilities|FlowControl|DoOnce false
        (:Completed
          (bind _outactors (Actor|GetAllActorsOfClass "BP_Key_C"))
          (bind _result (Math|Integer|IncrementInt (Variables|/Game/StealthGameAIKit/Characters/Player/BP_Player.BP_Player_C|GetCollectableCount PlayerPawn))
            (:%20%20
              (if (== _result (Utilities|Array|Length _outactors))
                (bind _output_get (Variables|Default|Setcount -1))
                (Default|UpdateObjective _mainwidget _output_get)
                (else
                  (CallFunction|ShowMarker _result)
                  (Default|UpdateObjective _mainwidget _result))))))))))

(event EventTick
  (params (DeltaSeconds :type Float%20%28single-precision%29))
  ;[1 1 1] Update the distance at each tick
  (Transformation|AddRelativeRotation (Variables|Default|GetStaticMesh) "0.000000,7.000000, 0" false false)
  (bind _aswbp_marker (Utilities|Casting|CastToWBP_Marker (UserInterface|GetWidget (Variables|Default|GetWidget))))
  (bind _returnvalue (Default|UpdateDistanceText _aswbp_marker (Transformation|GetWorldLocation (Variables|Default|GetStaticMesh))))
  (Default|UpdateScale _aswbp_marker (Math|Float|MapRangeClamped (Math|Conversions|ToFloat(Integer) _returnvalue) 0.0 1e+04 1.0 0.1) (Math|Float|MapRangeClamped (Math|Conversions|ToFloat(Integer) _returnvalue) 0.0 1e+04 1.0 0.1)))

(fn ConstructionScript
  (|CallParentFunction))

(fn ShowMarker
  (params (Index :type Integer))
  (bind _outactors (Actor|GetAllActorsOfClass "BP_Key_C"))
  (CallFunction|ShowWidget (Utilities|Array|Get(acopy) _outactors Index)))