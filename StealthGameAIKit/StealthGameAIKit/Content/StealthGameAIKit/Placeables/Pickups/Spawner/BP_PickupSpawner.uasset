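; Placeable pickup spawner that provides a respawning pickup of a configurable class.
; On BeginPlay it spawns the pickup at its SpawnLocation component, keeps a reference and binds Respawn to the pickup's OnPickuped event.
; Respawn deactivates that pickup and reactivates it after RespawnTime, reusing the same actor instead of spawning a new one.
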(event Custom|Respawn
  (Default|Deactivate (Variables|Reference|GetPickupRef))
  (Utilities|FlowControl|Delay (Variables|Config|GetRespawnTime))
  (Default|Activate (Variables|Reference|GetPickupRef)))

(event EventBeginPlay
  (bind _returnvalue (Game|SpawnActorfromClass (Variables|Config|GetSpawnPickupClass) (Transformation|GetWorldTransform (Variables|Default|GetSpawnLocation)) "AdjustIfPossibleButAlwaysSpawn" 0 0))
  (bind _output_get (Variables|Reference|SetPickupRef _returnvalue))
  (EventDispatchers|BindEventtoOnPickuped _output_get (delegate Custom|Respawn)))

(fn ConstructionScript)