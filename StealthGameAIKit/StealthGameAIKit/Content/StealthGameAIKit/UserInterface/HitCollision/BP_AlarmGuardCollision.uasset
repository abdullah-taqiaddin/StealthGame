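; BP_AlarmGuardCollision is a trigger volume that shows the player a timed tutorial hint about yellow alarm guards and disabling alarms.
; When BP_Player first overlaps the box, a DoOnce gate starts the sequence on that player's HintWidget.
; Delays step through two messages, then the widget's hint animation plays in reverse and HasBeenShown is set.
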(event OnComponentBeginOverlap(Box)
  (params (OverlappedComponent :type Primitive%20Component%20Object%20Reference) (OtherActor :type Actor%20Object%20Reference) (OtherComp :type Primitive%20Component%20Object%20Reference) (OtherBodyIndex :type Integer) (bFromSweep :type Boolean) (SweepResult :type Hit%20Result%20Structure%20%28by%20ref%29))
  (bind _asbp_player (Utilities|Casting|CastToBP_Player OtherActor))
  (Variables|Default|SetAs%20BP%20Player _asbp_player)
  (Utilities|FlowControl|DoOnce false
    (:Completed
      (Default|UpdateHint (Variables|/Game/StealthGameAIKit/Characters/Player/BP_Player.BP_Player_C|GetHintWidget (Variables|Default|GetAs%20BP%20Player)) "Guards dressed in yellow will instantly detect you and will set off an alarm that'll notify nearby guards.")
      (Utilities|FlowControl|Delay 1e+01)
      (Default|UpdateHint (Variables|/Game/StealthGameAIKit/Characters/Player/BP_Player.BP_Player_C|GetHintWidget (Variables|Default|GetAs%20BP%20Player)) "You can disable the alarm by getting close to it and pressing T.")
      (Utilities|FlowControl|Delay 5.0)
      (UserInterface|Animation|PlayAnimation (Variables|/Game/StealthGameAIKit/Characters/Player/BP_Player.BP_Player_C|GetHintWidget (Variables|Default|GetAs%20BP%20Player)) (Variables|/Game/StealthGameAIKit/UserInterface/WBP_Hint.WBP_Hint_C|GetHintAnimation (Variables|/Game/StealthGameAIKit/Characters/Player/BP_Player.BP_Player_C|GetHintWidget (Variables|Default|GetAs%20BP%20Player))) 0.0 1 "Reverse" 1.0 false)
      (Variables|Default|SetHasBeenShown true))))

(event EventBeginPlay)

(event Collision|EventActorBeginOverlap
  (params (OtherActor :type Actor%20Object%20Reference)))

(event EventTick
  (params (DeltaSeconds :type Float%20%28single-precision%29)))

(fn ConstructionScript)